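; StateMachineComponent is a skeleton state machine component that tracks a current state, with hooks for entering and exiting states.
; SetStateFunc stores the requested state, then calls OnExitState with a fixed Idle value if it differs from the current one.
; Only when the requested state matches does it set CurrentState and call OnEnterStateFunc with the target location and actor.
; Both hooks switch on state but have no case logic, and BeginPlay and Tick are unused.
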(event EventBeginPlay)

(event EventTick
  (params (DeltaSeconds :type Float%20%28single-precision%29)))

(fn SetStateFunc
  (params (StateToTransitionTo :type EUnitState%20Enum :default "NewEnumerator0") (TargetLocation :type Vector) (TargetActor :type Actor%20Object%20Reference))
  (LocalVariables|SetNewState StateToTransitionTo)
  (if (Utilities|Enum|NotEqual(Enum) StateToTransitionTo (Variables|Default|GetCurrentState))
    (CallFunction|OnExitState "NewEnumerator0")
    (else
      (bind _output_get (Variables|Default|SetCurrentState (LocalVariables|GetNewState)))
      (CallFunction|OnEnterStateFunc _output_get TargetLocation TargetActor))))

(fn OnEnterStateFunc
  (params (NewState :type EUnitState%20Enum :default "NewEnumerator0") (TargetLocation :type Vector) (TargetActor :type Actor%20Object%20Reference))
  (switch Utilities|FlowControl|Switch|SwitchonEUnitState NewState))

(fn OnExitState
  (params (State :type EUnitState%20Enum :default "NewEnumerator0"))
  (switch Utilities|FlowControl|Switch|SwitchonEUnitState State))