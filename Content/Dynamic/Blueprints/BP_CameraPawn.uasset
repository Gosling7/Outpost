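; BP_CameraPawn is a camera pawn with leftover edge-scroll logic for an RTS-style view, none of which currently runs.
; The MouseX and MouseY events are empty, and the disconnected logic sits under a comment marked "Old".
; That logic compares cursor position to viewport size and, near a screen edge, offsets the pawn in world X or Y by CameraSpeed scaled with delta time.
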(event Input|MouseEvents|MouseX
  (params (AxisValue :type Float%20%28single-precision%29))
  ;[0.15 0.15 0.15 0.5] Old
)

(event Input|MouseEvents|MouseY
  (params (AxisValue :type Float%20%28single-precision%29))
  ;[0.15 0.15 0.15 0.5] Old
)

(fn ConstructionScript)