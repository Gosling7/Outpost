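; BP_B_BuildingBase is a base building Blueprint that handles selection feedback and notifies actors that overlap it.
; On BeginPlay it creates a selected-building widget linked to itself, which select and deselect events show or remove along with a selector decal.
; Overlapping actors receive a DropoffMessage call.
; Location, attack-move, resource count and unit-grab functions are stubs returning empty or default values.
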(event Collision|EventActorBeginOverlap
  (params (OtherActor :type Actor%20Object%20Reference))
  (Class|BPIResource|Dropoff(Message) OtherActor))

(event EventTick
  (params (DeltaSeconds :type Float%20%28single-precision%29)))

(event EventSelectThis
  (Rendering|SetVisibility (Variables|Default|GetSelectorDecal) true false)
  (UserInterface|Viewport|AddtoViewport (Variables|Default|GetSelectedBuildingWidget) 0))

(event EventDeselectThis
  (Rendering|SetVisibility (Variables|Default|GetSelectorDecal) false false)
  (Widget|RemovefromParent (Variables|Default|GetSelectedBuildingWidget)))

(event EventBeginPlay
  (bind _returnvalue (UserInterface|CreateWidget "/Game/Dynamic/Blueprints/WBP_SelectedBuilding.WBP_SelectedBuilding_C"))
  (bind _output_get (Variables|Default|SetSelectedBuildingWidget _returnvalue))
  (Variables|/Game/Dynamic/Blueprints/WBP_SelectedBuilding.WBP_SelectedBuilding_C|SetSelectedBuilding _output_get self))

(fn ConstructionScript)

(fn FindValidLocation
  (params (TargetLocation :type Vector :default "0, 0, 0") (TargetActor :type Actor%20Object%20Reference))
  (return "0, 0, 0"))

(fn GetIsAttackMoveCommand
  (return false))

(fn GetResourceCount
  (return 0))

(fn GrabSelectedUnits
  (return 0))