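; Player state Blueprint that tracks a player's Wood and Food, seeded from StartingResources in the construction script.
; Increase and decrease events call AddResources and RemoveResources, which rebuild CurrentResources and push it to the resources widget.
; BeginPlay takes that widget from player controller 0, cast to BP_ControllerNew.
; HasEnoughResources returns true when either Wood or Food covers its cost, not necessarily both, and RemoveResources subtracts without checking.
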(event EventIncreasePlayerResources
  (params (ToAdd :type F%20Resource%20Structure))
  (CallFunction|AddResources (.type ToAdd) (.amount ToAdd)))

(event EventDecreasePlayerResources
  (params (Cost :type F%20Player%20Resources%20Structure))
  (CallFunction|RemoveResources Cost))

(event EventBeginPlay
  (bind _asbp_controller_new (Utilities|Casting|CastToBP_ControllerNew (Game|GetPlayerController 0)))
  (Variables|Default|SetResourcesWidget (Variables|/Game/Blueprints/BP_ControllerNew.BP_ControllerNew_C|GetResourcesWidget _asbp_controller_new)))

(fn ConstructionScript
  (Variables|Default|SetCurrentResources (Variables|Default|GetStartingResources)))

(fn AddResources
  (params (Type :type EResourceType%20Enum :default "NewEnumerator0") (Amount :type Integer))
  (Utilities|FlowControl|Sequence
    (:then_0
      (LocalVariables|SetamountToAdd Amount)
      (LocalVariables|SetcurrentWood (.Amount (Utilities|Struct|BreakF_Resource (.wood (Variables|Default|GetCurrentResources)))))
      (LocalVariables|SetcurrentFood (.Amount (Utilities|Struct|BreakF_Resource (.food (Variables|Default|GetCurrentResources))))))
    (:then_1
      (switch Utilities|FlowControl|Switch|SwitchonEResourceType Type
        (:NewEnumerator0
          (Variables|Default|SetCurrentResources (Utilities|Struct|MakeF_PlayerResources (Utilities|Struct|MakeF_Resource "NewEnumerator0" (+ (LocalVariables|GetcurrentWood) (LocalVariables|GetamountToAdd))) (Utilities|Struct|MakeF_Resource "NewEnumerator1" (LocalVariables|GetcurrentFood)) "(Type_7_7A3CDB9048DB4B18273B9DB90D6CAA69=NewEnumerator0,Amount_9_4083E1D34259B6D59F8C98ADB0DA72C0=0)" "(Type_7_7A3CDB9048DB4B18273B9DB90D6CAA69=NewEnumerator0,Amount_9_4083E1D34259B6D59F8C98ADB0DA72C0=0)")))
        (:NewEnumerator1
          (Variables|Default|SetCurrentResources (Utilities|Struct|MakeF_PlayerResources (Utilities|Struct|MakeF_Resource "NewEnumerator0" (LocalVariables|GetcurrentWood)) (Utilities|Struct|MakeF_Resource "NewEnumerator1" (+ (LocalVariables|GetcurrentFood) (LocalVariables|GetamountToAdd))) "(Type_7_7A3CDB9048DB4B18273B9DB90D6CAA69=NewEnumerator0,Amount_9_4083E1D34259B6D59F8C98ADB0DA72C0=0)" "(Type_7_7A3CDB9048DB4B18273B9DB90D6CAA69=NewEnumerator0,Amount_9_4083E1D34259B6D59F8C98ADB0DA72C0=0)"))))
      (Class|BIHUD|UpdateResourcesWidget(Message) (Variables|Default|GetResourcesWidget) (Variables|Default|GetCurrentResources)))))

(fn RemoveResources
  (params (Cost :type F%20Player%20Resources%20Structure))
  (bind (_wood _food) (Utilities|Struct|BreakF_PlayerResources Cost))
  (Utilities|FlowControl|Sequence
    (:then_0
      (LocalVariables|SetcurrentWood (.Amount (Utilities|Struct|BreakF_Resource (.wood (Variables|Default|GetCurrentResources)))))
      (LocalVariables|SetcurrentFood (.Amount (Utilities|Struct|BreakF_Resource (.food (Variables|Default|GetCurrentResources)))))
      (LocalVariables|SetcostWood (.Amount (Utilities|Struct|BreakF_Resource _wood)))
      (LocalVariables|SetcostFood (.Amount (Utilities|Struct|BreakF_Resource _food))))
    (:then_1
      (bind _output_get (Variables|Default|SetCurrentResources (Utilities|Struct|MakeF_PlayerResources (Utilities|Struct|MakeF_Resource "NewEnumerator0" (- (LocalVariables|GetcurrentWood) (LocalVariables|GetcostWood))) (Utilities|Struct|MakeF_Resource "NewEnumerator1" (- (LocalVariables|GetcurrentFood) (LocalVariables|GetcostFood))) "(Type_7_7A3CDB9048DB4B18273B9DB90D6CAA69=NewEnumerator0,Amount_9_4083E1D34259B6D59F8C98ADB0DA72C0=0)" "(Type_7_7A3CDB9048DB4B18273B9DB90D6CAA69=NewEnumerator0,Amount_9_4083E1D34259B6D59F8C98ADB0DA72C0=0)")))
      (Class|BIHUD|UpdateResourcesWidget(Message) (Variables|Default|GetResourcesWidget) _output_get))))

(fn HasEnoughResources
  (params (Cost :type F%20Player%20Resources%20Structure))
  (bind (_wood _food) (Utilities|Struct|BreakF_PlayerResources Cost))
  (Utilities|FlowControl|Sequence
    (:then_0
      (LocalVariables|SetcurrentWood (.Amount (Utilities|Struct|BreakF_Resource (.wood (Variables|Default|GetCurrentResources)))))
      (LocalVariables|SetcurrentFood (.Amount (Utilities|Struct|BreakF_Resource (.food (Variables|Default|GetCurrentResources)))))
      (LocalVariables|SetcostWood (.Amount (Utilities|Struct|BreakF_Resource _wood)))
      (LocalVariables|SetcostFood (.Amount (Utilities|Struct|BreakF_Resource _food))))
    (:then_1
      (if (or (<= (LocalVariables|GetcostWood) (LocalVariables|GetcurrentWood)) (<= (LocalVariables|GetcostFood) (LocalVariables|GetcurrentFood)))
        (return true)
        (else
          (return false))))))