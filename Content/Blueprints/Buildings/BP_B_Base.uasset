(event Custom|CustomEvent
  (if (Utilities|Array|IsNotEmpty (Variables|Construction|GetActiveBuilders))
    (if (< (Variables|Construction|GetBuildProgress) (Variables|Construction|GetNeededConstructionPoints))
      (Variables|Construction|SetBuildProgress (+ (Variables|Construction|GetBuildProgress) 1.0))
      (else
        (Utilities|Time|ClearandInvalidateTimerbyHandle (Variables|Construction|GetBuildTimer))
        (Variables|Default|SetbIsUnderConstruction false)
        (Rendering|SetVisibility (Variables|Default|GetUnderConstructionMesh) false false)
        (Rendering|SetVisibility (Variables|Default|GetBuildingMesh) true false)
        (Rendering|Material|SetMaterial (Variables|Default|GetBuildingMesh) 0 "/Engine/EngineMaterials/WorldGridMaterial.WorldGridMaterial")
        (for _array_element (Variables|Construction|GetActiveBuilders)
          (Class|BIWorkerUnit|BuildingCompleted(Message) _array_element))))))

(event Collision|EventActorBeginOverlap
  (params (OtherActor :type Actor%20Object%20Reference))
  (Class|BIResourceNode|Dropoff(Message) OtherActor))

(event EventRemovefromActiveBuilders
  (params (Worker :type Actor%20Object%20Reference))
  (Utilities|Array|RemoveItem (Variables|Construction|GetActiveBuilders) Worker)
  (if (Utilities|Array|IsEmpty (Variables|Construction|GetActiveBuilders))
    (Utilities|Time|ClearandInvalidateTimerbyHandle (Variables|Construction|GetBuildTimer))))

(event EventTick
  (params (DeltaSeconds :type Float%20%28single-precision%29)))

(event EventBeginPlay
  (bind _returnvalue (UserInterface|CreateWidget "/Game/Blueprints/Widgets/WBP_SelectedBuilding.WBP_SelectedBuilding_C"))
  (bind _output_get (Variables|Default|SetSelectedBuildingWidget _returnvalue))
  (Variables|/Game/Blueprints/Widgets/WBP_SelectedBuilding.WBP_SelectedBuilding_C|SetSelectedBuilding _output_get self))

(event EventAddtoActiveBuilders
  (params (Worker :type Actor%20Object%20Reference))
  (Utilities|Array|AddUnique (Variables|Construction|GetActiveBuilders) Worker))

(event EventBuild
  (Variables|Default|SetbIsUnderConstruction true)
  (bind _returnvalue (Utilities|Time|SetTimerbyEvent (delegate Custom|CustomEvent) 1.0 true))
  (Variables|Construction|SetBuildTimer _returnvalue))

(fn ConstructionScript)

(fn GetActiveBuilders
  (return (Variables|Construction|GetActiveBuilders)))

(fn GetIsUnderConstruction
  (return (Variables|Default|GetbIsUnderConstruction)))