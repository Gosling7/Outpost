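; Base RTS-style unit that shows a selection decal and takes move and attack commands, caching its AI controller on BeginPlay.
; Command events delegate to the UnitMovement and UnitCombat components, while other events append to, clear or recheck the command queue.
; HandleCommandQueue dispatches the first entry by type without removing it here.
; Local move/attack enqueue functions, including move-before-attack when out of range, are only called from unwired nodes in this graph.
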(event EventBeginPlay
  (Variables|Default|SetAIController (AI|GetAIController self)))

(event EventAttackCommand
  (params (TargetActor :type Actor%20Object%20Reference) (TargetLocation :type Vector :default "0, 0, 0"))
  (bind _unitcombat (Variables|Default|GetUnitCombat))
  (Default|HandleAttackCommand _unitcombat TargetLocation TargetActor self (Variables|/Game/Blueprints/Components/UnitCombat.UnitCombat_C|GetAttack%20Range _unitcombat)))

(event EventMoveCommand
  (params (TargetLocation :type Vector :default "0, 0, 0") (TargetActor :type Actor%20Object%20Reference))
  (Default|HandleMoveCommand (Variables|Default|GetUnitMovement) (Variables|Default|GetAIController) TargetLocation TargetActor self (Variables|Default|GetCommandQueue)))

(event EventAddCommandstoQueue
  (params (Command :type Array%20of%20F%20Unit%20Command%20Structures))
  (Utilities|Array|AppendArray (Variables|Default|GetCommandQueue) Command))

(event EventClearCommandQueue
  (Utilities|Array|Clear (Variables|Default|GetCommandQueue)))

(event EventCheckCommandQueue
  (CallFunction|HandleCommandQueue (Variables|Default|GetCommandQueue)))

(event EventSetSelected
  (params (Value :type Boolean))
  (bind _selectordecal (Variables|Default|GetSelectorDecal))
  (if Value
    (Rendering|SetVisibility _selectordecal true false)
    (else
      (Rendering|SetVisibility _selectordecal false false))))

(fn ConstructionScript)

(fn HandleMoveCommand
  (params (TargetLocation :type Vector))
  (bind _commandqueue (Variables|Default|GetCommandQueue))
  (Utilities|Array|Add _commandqueue (Utilities|Struct|MakeF_UnitCommand "NewEnumerator0" TargetLocation 0))
  (CallFunction|HandleCommandQueue _commandqueue))

(fn HandleAttackCommand
  (params (TargetActor :type Actor%20Object%20Reference) (TargetLocation :type Vector))
  (Utilities|FlowControl|Sequence
    (:then_0
      (LocalVariables|SetAttackTarget TargetActor)
      (LocalVariables|SetAttackTargetLocation TargetLocation))
    (:then_1
      (if (<= (Transformation|GetDistanceTo TargetActor) (Variables|/Game/Blueprints/Components/UnitCombat.UnitCombat_C|GetAttack%20Range (Variables|Default|GetUnitCombat)))
        (Utilities|Array|Add (Variables|Default|GetCommandQueue) (Utilities|Struct|MakeF_UnitCommand "NewEnumerator1" (LocalVariables|GetAttackTargetLocation) (LocalVariables|GetAttackTarget)))
        (else
          (Utilities|Array|Add (Variables|Default|GetCommandQueue) (Utilities|Struct|MakeF_UnitCommand "NewEnumerator0" (LocalVariables|GetAttackTargetLocation) (LocalVariables|GetAttackTarget)))
          (Utilities|Array|Add (Variables|Default|GetCommandQueue) (Utilities|Struct|MakeF_UnitCommand "NewEnumerator1" (LocalVariables|GetAttackTargetLocation) (LocalVariables|GetAttackTarget)))))
      (CallFunction|HandleCommandQueue (Variables|Default|GetCommandQueue)))))

(fn HandleCommandQueue
  (params (CommandQueue :type Array%20of%20F%20Unit%20Command%20Structures))
  (if (Utilities|Array|IsNotEmpty CommandQueue)
    (bind _output_get (LocalVariables|SetCurrentCommand (Utilities|Array|Get(acopy) CommandQueue)))
    (switch Utilities|FlowControl|Switch|SwitchonEUnitCommand (.commandtype _output_get)
      (:NewEnumerator0
        (CallFunction|HandleMoveCommandinQueue (Variables|Default|GetCommandQueue) (LocalVariables|GetCurrentCommand) (Variables|Default|GetUnitMovement) self (Variables|Default|GetAIController)))
      (:NewEnumerator1
        (CallFunction|HandleAttackCommandinQueue (Variables|Default|GetCommandQueue) (LocalVariables|GetCurrentCommand) (Variables|Default|GetUnitCombat) self (Variables|Default|GetAIController))))))

(fn GetBuildingtoBuild
  (return 0))

(fn GetUnitCommandQueue
  (return (Variables|Default|GetCommandQueue)))