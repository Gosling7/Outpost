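; Base RTS unit that takes move, attack and attack-move orders, with selection decals, a selected-unit widget and a health bar.
; Orders enter a command queue, processed by Idle/Moving/Attacking state into AI moves and timer-driven damage.
; Looping sphere traces auto-acquire the nearest target in aggro range, including during attack-moves.
; FindValidLocation resolves actor approach points through navmesh fallbacks; on death, the unit notifies actors targeting it.
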(event OnDeath(HealthComponent)
  (Development|PrintString "Friendly Unit DIED!")
  (for _array_element (Variables|Combat|GetTargetedByActors)
    (Class|BPIDamageable|RemoveUnitfromEnemyTarget(Message) _array_element))
  (Actor|DestroyActor))

(event OnDamageTaken(HealthComponent)
  (Development|PrintString (Utilities|String|Append "Current Friendly Unit Health: " (Utilities|String|ToString(Float) (Variables|/Game/Blueprints/Components/HealthComponent.HealthComponent_C|GetHealth (Variables|Default|GetHealthComponent))))))

(event Custom|ExecuteMoveCommand
  (bind _currentcommand (Variables|FSM|GetCurrentCommand))
  (Utilities|Array|RemoveItem (Variables|FSM|GetCommandQueue) (Variables|FSM|GetCurrentCommand))
  (Utilities|Time|ClearandInvalidateTimerbyHandle (Variables|FSM|GetTryAttackTimer))
  (Utilities|Time|ClearandInvalidateTimerbyHandle (Variables|FSM|GetLookForNearbyTargetTimer))
  (Variables|FSM|SetCurrentState "NewEnumerator1")
  (AI|Navigation|StopMovement (Variables|Default|GetAIController))
  (Utilities|IsValid (.targetactor _currentcommand)
    (:Is%20Valid
      (bind _validlocation (CallFunction|FindValidLocation "0, 0, 0" (.targetactor _currentcommand)))
      (AI|AIMoveTo (Variables|Default|GetAIController) _validlocation 0 (Variables|Navigation|GetAcceptance%20Radius) "Default" "Default" true true
        (:OnMoveFinished
          _)))
    (:Is%20Not%20Valid
      (bind _validlocation_2 (CallFunction|FindValidLocation (.targetlocation _currentcommand)))
      (AI|AIMoveTo (Variables|Default|GetAIController) _validlocation_2 0 (Variables|Navigation|GetAcceptance%20Radius) "Default" "Default" true true
        (:OnMoveFinished
          _))))
  (Variables|FSM|SetCurrentState "NewEnumerator0")
  (if (Class|KismetMathLibrary|IsNearlyZero2D (Math|Conversions|ToVector2D(Vector) (- (Transformation|GetActorLocation) (Variables|Default|GetTargetLocation))) 1e+02)
    (CallFunction|LookforNearbyTarget))
  (CallFunction|TryProcessNextCommand))

(event Custom|TryProcessNextCommand
  (switch Utilities|FlowControl|Switch|SwitchonEUnitState (Variables|FSM|GetCurrentState)
    (:NewEnumerator0
      (if (Utilities|Array|IsNotEmpty (Variables|FSM|GetCommandQueue))
        (bind _output_get (Variables|FSM|SetCurrentCommand (Utilities|Array|Get(acopy) (Variables|FSM|GetCommandQueue))))
        (switch Utilities|FlowControl|Switch|SwitchonEUnitCommand (.CommandType (Utilities|Struct|BreakF_UnitCommand _output_get))
          (:NewEnumerator0
            (CallFunction|ExecuteMoveCommand))
          (:NewEnumerator1
            (CallFunction|ExecuteAttackCommand))
          (:NewEnumerator2
            (CallFunction|ExecuteAttackMoveCommand)))))
    (:NewEnumerator1
      (if (> (Utilities|Array|Length (Variables|FSM|GetCommandQueue)) 1)
        (bind _array_element (Utilities|Array|ForEachLoopwithBreak (Variables|FSM|GetCommandQueue) :!label _label)
          (:LoopBody
            (if (Utilities|Enum|Equal(Enum) (.CommandType (Utilities|Struct|BreakF_UnitCommand _array_element)) "NewEnumerator1")
              (Utilities|Array|RemoveItem (Variables|FSM|GetCommandQueue) _array_element)
              (goto _label Break)))
          (:Completed
            (bind _output_get_2 (Variables|FSM|SetCurrentCommand (Utilities|Array|Get(acopy) (Variables|FSM|GetCommandQueue)) :!label _label_2))
            (switch Utilities|FlowControl|Switch|SwitchonEUnitCommand (.CommandType (Utilities|Struct|BreakF_UnitCommand _output_get_2))
              (:NewEnumerator0
                (CallFunction|ExecuteMoveCommand))
              (:NewEnumerator1
                (CallFunction|ExecuteAttackCommand))
              (:NewEnumerator2
                (CallFunction|ExecuteAttackMoveCommand)))))
        (else
          (goto _label_2))))
    (:NewEnumerator2
      (bind _output_get_3 (Variables|FSM|SetCurrentCommand (Utilities|Array|Get(acopy) (Variables|FSM|GetCommandQueue))))
      (switch Utilities|FlowControl|Switch|SwitchonEUnitCommand (.CommandType (Utilities|Struct|BreakF_UnitCommand _output_get_3))
        (:NewEnumerator0
          (CallFunction|ExecuteMoveCommand))
        (:NewEnumerator1
          (CallFunction|ExecuteAttackCommand))
        (:NewEnumerator2
          (CallFunction|ExecuteAttackMoveCommand))))))

(event Custom|LookForNearbyTargetDuringAttackMove
  (bind _returnvalue (Utilities|Time|SetTimerbyEvent (delegate Custom|LookWhileAttackMove) 0.1 true))
  (Variables|FSM|SetLookForNeabyTargetDuringAttackMoveTimer _returnvalue))

(event Custom|CustomEvent
  (bind _targetactor (Variables|FSM|GetTargetActor))
  (Utilities|IsValid _targetactor
    (:Is%20Valid
      (if (not (>= (Transformation|GetDistanceTo _targetactor) (Variables|FSM|GetAttackRange)))
        (Game|Damage|ApplyDamage (Variables|FSM|GetTargetActor) (Variables|FSM|GetAttackDamage) (Variables|Default|GetAIController) 0)))
    (:Is%20Not%20Valid
      (Utilities|Time|ClearandInvalidateTimerbyHandle (Variables|Default|GetTryAttackDuringAttackMoveTImer))
      (CallFunction|LookforNearbyTargetDuringAttackMove)
      (AI|AIMoveTo (Variables|Default|GetAIController) (Variables|FSM|GetAttackMoveTargetLocation) 0 (Variables|Navigation|GetAcceptance%20Radius) "Default" "Default" true true
        (:OnMoveFinished
          (Utilities|Time|ClearandInvalidateTimerbyHandle (Variables|FSM|GetLookForNeabyTargetDuringAttackMoveTimer))
          (Variables|FSM|SetCurrentState "NewEnumerator0"))))))

(event Custom|TryAttack
  (bind _targetactor (Variables|FSM|GetTargetActor))
  (Utilities|IsValid _targetactor
    (:Is%20Valid
      (if (>= (Transformation|GetDistanceTo _targetactor) (Variables|FSM|GetAttackRange))
        (Utilities|Time|ClearandInvalidateTimerbyHandle (Variables|FSM|GetTryAttackTimer))
        (if (Variables|FSM|GetbIsDuringAttackMove)
          (Utilities|Array|Add (Variables|FSM|GetCommandQueue) (Utilities|Struct|MakeF_UnitCommand "NewEnumerator0" (Variables|Default|GetTargetLocation) 0))
          (CallFunction|TryProcessNextCommand)
          (else
            (Utilities|Array|Add (Variables|FSM|GetCommandQueue) (Utilities|Struct|MakeF_UnitCommand "NewEnumerator0" "0.000000,0.000000,0.000000" (Variables|FSM|GetTargetActor)))
            (Utilities|Array|Add (Variables|FSM|GetCommandQueue) (Utilities|Struct|MakeF_UnitCommand "NewEnumerator1" "0.000000,0.000000,0.000000" (Variables|FSM|GetTargetActor)))
            (CallFunction|TryProcessNextCommand)))
        (else
          (Game|Damage|ApplyDamage (Variables|FSM|GetTargetActor) (Variables|FSM|GetAttackDamage) (Variables|Default|GetAIController) 0))))
    (:Is%20Not%20Valid
      (Utilities|Time|ClearandInvalidateTimerbyHandle (Variables|FSM|GetTryAttackTimer))
      (if (Variables|FSM|GetbIsDuringAttackMove)
        (Utilities|Array|Add (Variables|FSM|GetCommandQueue) (Utilities|Struct|MakeF_UnitCommand "NewEnumerator0" (Variables|FSM|GetAttackMoveTargetLocation) 0))
        (CallFunction|TryProcessNextCommand)
        (else
          (CallFunction|LookforNearbyTarget))))))

(event Custom|ExecuteAttackCommand
  (Variables|FSM|SetTargetActor (.targetactor (Variables|FSM|GetCurrentCommand)))
  (Utilities|Array|RemoveItem (Variables|FSM|GetCommandQueue) (Variables|FSM|GetCurrentCommand))
  (Variables|FSM|SetCurrentState "NewEnumerator2")
  (bind _returnvalue (Utilities|Time|SetTimerbyEvent (delegate Custom|TryAttack) (Variables|FSM|GetAttackSpeed) true))
  (Variables|FSM|SetTryAttackTimer _returnvalue))

(event Custom|LookUntilReachedLocation
  (if (< (.PathLength (Class|NavigationSystemV1|GetPathLength (Transformation|GetActorLocation (Variables|Default|GetAIController)) (Variables|FSM|GetAttackMoveTargetLocation) 0 0)) 1e+01)
    (Utilities|Time|ClearandInvalidateTimerbyHandle (Variables|Default|GetLookUntilReachedLocationTimer))
    (Utilities|Time|ClearandInvalidateTimerbyHandle (Variables|FSM|GetLookForNeabyTargetDuringAttackMoveTimer))
    (Variables|FSM|SetCurrentState "NewEnumerator0")))

(event Custom|LookWhileAttackMove
  (Utilities|LookforNeabyTargetMacro
    (:Found
      (Development|PrintString "LookForNearbyTargetDuringAttackMove Found path")
      (Utilities|Time|ClearandInvalidateTimerbyHandle (Variables|FSM|GetLookForNeabyTargetDuringAttackMoveTimer))
      (AI|Navigation|StopMovement (Variables|Default|GetAIController))
      (bind _validlocation (CallFunction|FindValidLocation "0, 0, 0" (Variables|FSM|GetTargetActor)))
      (AI|AIMoveTo (Variables|Default|GetAIController) _validlocation 0 (Variables|Navigation|GetAcceptance%20Radius) "Default" "Default" true true
        (:OnMoveFinished
          (bind _returnvalue (Utilities|Time|SetTimerbyEvent (delegate Custom|CustomEvent) 1.0 true))
          (Variables|Default|SetTryAttackDuringAttackMoveTImer _returnvalue))))
    (:NotFound
      (Development|PrintString "LookForNearbyTargetDuringAttackMove Not Found path"))))

(event Custom|ExecuteAttackMoveCommand
  (Utilities|Time|ClearandInvalidateTimerbyHandle (Variables|FSM|GetLookForNearbyTargetTimer))
  (AI|Navigation|StopMovement (Variables|Default|GetAIController))
  (Utilities|Array|RemoveItem (Variables|FSM|GetCommandQueue) (Variables|FSM|GetCurrentCommand))
  (bind _validlocation (CallFunction|FindValidLocation (Variables|FSM|GetAttackMoveTargetLocation)))
  (AI|AIMoveTo (Variables|Default|GetAIController) _validlocation 0 (Variables|Navigation|GetAcceptance%20Radius) "Default" "Default" true true
    (:then
      (CallFunction|LookforNearbyTargetDuringAttackMove)
      (Variables|FSM|SetCurrentState "NewEnumerator1"))))

(event Custom|LookForNearbyTarget
  (Utilities|Time|ClearandInvalidateTimerbyHandle (Variables|FSM|GetLookForNearbyTargetTimer))
  (bind _returnvalue (Utilities|Time|SetTimerbyEvent (delegate Custom|Look) 1.0 true))
  (Variables|FSM|SetLookForNearbyTargetTimer _returnvalue))

(event Custom|Look
  (Utilities|LookforNeabyTargetMacro
    (:Found
      (Development|PrintString "LookForNearbyTarget Found path")
      (Utilities|Time|ClearandInvalidateTimerbyHandle (Variables|FSM|GetLookForNearbyTargetTimer))
      (Utilities|Array|Add (Variables|FSM|GetCommandQueue) (Utilities|Struct|MakeF_UnitCommand "NewEnumerator0" "0.000000,0.000000,0.000000" (Variables|FSM|GetTargetActor)))
      (Utilities|Array|Add (Variables|FSM|GetCommandQueue) (Utilities|Struct|MakeF_UnitCommand "NewEnumerator1" "0.000000,0.000000,0.000000" (Variables|FSM|GetTargetActor)))
      (CallFunction|TryProcessNextCommand))
    (:NotFound
      (Development|PrintString "LookForNearbyTarget Not Found path"))))

(event EventBeginPlay
  ;[0.15 0.15 0.15 0.5] Setup Selected Unit Widget
  (Variables|Default|SetAIController (AI|GetAIController self))
  (Variables|Default|SetRTSController (Game|GetPlayerController 0))
  (bind _returnvalue (UserInterface|CreateWidget "/Game/Blueprints/Widgets/WBP_SelectedUnit.WBP_SelectedUnit_C"))
  (bind _output_get (Variables|Default|SetSelectedUnitWidget _returnvalue))
  (Variables|/Game/Blueprints/Widgets/WBP_SelectedUnit.WBP_SelectedUnit_C|SetUnitReferance _output_get self)
  (Appearance|SetBrushfromTexture (Variables|/Game/Blueprints/Widgets/WBP_SelectedUnit.WBP_SelectedUnit_C|GetUnitImage _returnvalue) (Variables|Default|Get2DImage) false)
  (bind _output_get_2 (Variables|Default|SetHealthBar (UserInterface|GetWidget (Variables|Default|GetHealthBarWidget))))
  (Default|SetupHealthBar (Variables|Default|GetHealthComponent) _output_get_2)
  (CallFunction|LookforNearbyTarget))

(event EventAttackMoveCommand
  (params (TargetLocation :type Vector :default "0, 0, 0"))
  (Variables|Default|SetIsInAttackMove true)
  (bind _output_get (Variables|FSM|SetAttackMoveTargetLocation TargetLocation))
  (Utilities|Array|Add (Variables|FSM|GetCommandQueue) (Utilities|Struct|MakeF_UnitCommand "NewEnumerator2" _output_get 0))
  (CallFunction|TryProcessNextCommand))

(event EventAddEnemytoTargetedbyActors
  (params (EnemyActor :type Actor%20Object%20Reference))
  (Utilities|Array|AddUnique (Variables|Combat|GetTargetedByActors) EnemyActor))

(event EventAttackCommand
  (params (TargetActor :type Actor%20Object%20Reference))
  (bind _output_get (Variables|FSM|SetTargetActor TargetActor))
  (if (>= (Transformation|GetDistanceTo _output_get) (Variables|FSM|GetAttackRange))
    (Utilities|Array|Add (Variables|FSM|GetCommandQueue) (Utilities|Struct|MakeF_UnitCommand "NewEnumerator0" "0.000000,0.000000,0.000000" TargetActor))
    (Utilities|Array|Add (Variables|FSM|GetCommandQueue) (Utilities|Struct|MakeF_UnitCommand "NewEnumerator1" "0.000000,0.000000,0.000000" TargetActor))
    (CallFunction|TryProcessNextCommand)
    (else
      (Utilities|Array|Add (Variables|FSM|GetCommandQueue) (Utilities|Struct|MakeF_UnitCommand "NewEnumerator1" "0.000000,0.000000,0.000000" TargetActor))
      (CallFunction|TryProcessNextCommand))))

(event EventSetSelected
  (params (Value :type Boolean))
  (bind _selectordecal (Variables|Default|GetSelectorDecal))
  (if Value
    (Rendering|SetVisibility _selectordecal true false)
    (else
      (Rendering|SetVisibility _selectordecal false false))))

(event EventSelectThis
  ;[0.15 0.15 0.15 0.5] Selection
  (Rendering|SetVisibility (Variables|Default|GetSelectorDecal) true false)
  (Class|BPIRTS|AddUnittoSelectedUnitsArea(Message) (Game|GetPlayerController 0) (Variables|Default|GetSelectedUnitWidget)))

(event EventDeselectThis
  ;[0.15 0.15 0.15 0.5] Selection
  (Rendering|SetVisibility (Variables|Default|GetSelectorDecal) false false)
  (Widget|RemovefromParent (Variables|Default|GetSelectedUnitWidget)))

(event EventHighlightUnit
  ;[0.15 0.15 0.15 0.5] Highlight
  (Rendering|Components|Decal|SetDecalMaterial (Variables|Default|GetSelectorDecal) "/Game/Materials/M_HighlightDecal.M_HighlightDecal"))

(event EventUnHighlightUnit
  ;[0.15 0.15 0.15 0.5] Highlight
  (Rendering|Components|Decal|SetDecalMaterial (Variables|Default|GetSelectorDecal) "/Game/Materials/M_SelectorDecal.M_SelectorDecal"))

(event Game|Damage|EventAnyDamage
  (params (Damage :type Float%20%28single-precision%29) (DamageType :type Damage%20Type%20Object%20Reference) (InstigatedBy :type Controller%20Object%20Reference) (DamageCauser :type Actor%20Object%20Reference))
  (Default|TakeDamage (Variables|Default|GetHealthComponent) Damage (Variables|Default|GetHealthBar))
  (Development|PrintString (Utilities|String|Append "Taken: " (Utilities|String|ToString(Float) Damage) " damage")))

(event EventMoveCommand
  (params (TargetLocation :type Vector :default "0, 0, 0"))
  (Variables|Default|SetTargetLocation TargetLocation)
  (Utilities|Array|Add (Variables|FSM|GetCommandQueue) (Utilities|Struct|MakeF_UnitCommand "NewEnumerator0" TargetLocation 0))
  (CallFunction|TryProcessNextCommand))

(fn ConstructionScript)

(fn FindValidLocation
  (params (TargetLocation :type Vector :default "0, 0, 0") (TargetActor :type Actor%20Object%20Reference))
  (Utilities|IsValid TargetActor
    (:Is%20Valid
      (Variables|Default|SetTargetLocation (Transformation|GetActorLocation TargetActor))
      (Variables|Default|SetDirectionToTarget (Class|KismetMathLibrary|VectorNormal2D (- (Variables|Default|GetTargetLocation) (Transformation|GetActorLocation)) 0.0001))
      (bind _output_get (Variables|Default|SetPreferredTargetLocation (- (Variables|Default|GetTargetLocation) (* (Variables|Default|GetDirectionToTarget) (Variables|Navigation|GetDirectionToTargetDistanceOffset) 0.5))))
      (bind _output_get_2 (Variables|Default|SetNearestValidPoint (.ProjectedLocation (AI|Navigation|ProjectPointtoNavigation (Class|NavigationSystemV1|GetNavigationSystem) _output_get 0 0 (Math|Conversions|ToVector(Float) (Variables|Navigation|GetValidPointSearchRadius))))))
      (if (.ReturnValue (AI|Navigation|ProjectPointtoNavigation (Class|NavigationSystemV1|GetNavigationSystem) _output_get 0 0 (Math|Conversions|ToVector(Float) (Variables|Navigation|GetValidPointSearchRadius))))
        (return _output_get_2)
        (else
          (bind _returnvalue (Class|NavigationSystemV1|FindPathtoLocationSynchronously (Transformation|GetActorLocation) (Variables|Default|GetTargetLocation) 0 0))
          (if (Utilities|IsValid _returnvalue)
            (bind _output_get_3 (Variables|Default|SetFinalPathPoint (Utilities|Array|Get(acopy) (Variables|/Script/NavigationSystem.NavigationPath|GetPathPoints _returnvalue) (Utilities|Array|LastIndex (Variables|/Script/NavigationSystem.NavigationPath|GetPathPoints _returnvalue)))))
            (return _output_get_3)
            (else
              (bind _output_get_4 (Variables|Default|SetExpandedTargetLocation (+ (* (Variables|Default|GetDirectionToTarget) (Variables|Navigation|GetDirectionToTargetDistanceOffset)) (Variables|Default|GetTargetLocation))))
              (bind _output_get_5 (Variables|Default|SetNearestValidPoint (.ProjectedLocation (AI|Navigation|ProjectPointtoNavigation _output_get_4 0 0 (Math|Conversions|ToVector(Float) (* (Variables|Navigation|GetValidPointSearchRadius) (Variables|Navigation|GetValidPointSearchRadiusMultiplier)))))))
              (if (.ReturnValue (AI|Navigation|ProjectPointtoNavigation _output_get_4 0 0 (Math|Conversions|ToVector(Float) (* (Variables|Navigation|GetValidPointSearchRadius) (Variables|Navigation|GetValidPointSearchRadiusMultiplier)))))
                (return _output_get_5)
                (else
                  (Development|PrintString "All navigation attempts failed. Worker cannot reach the tree!" true true "(R=1.000000,G=0.000000,B=0.000000,A=1.000000)"))))))))
    (:Is%20Not%20Valid
      (return TargetLocation))))

(fn GetIsAttackMoveCommand
  (return false))

(fn GetIsNodeDepleted
  (return false))

(fn GetIsNodeGatherable
  (return false))

(fn GetResourceCount
  (return 0))

(fn GetResourceLeft
  (return 0))

(fn GrabSelectedUnits
  (return 0))