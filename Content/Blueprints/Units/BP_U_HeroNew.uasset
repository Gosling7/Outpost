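; Player hero unit Blueprint that carries out queued move, attack, gather and drop-off commands.
; HandleCommandQueue switches on the first command's type and passes it to the matching handler with the movement, combat or gatherer component.
; Gather and find-new-resource events delegate to UnitGatherer.
; ClearCommandQueue empties the queue, stops AI movement and cancels the gather timer.
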(event EventFindNewResourceNode
  (Default|FindNewResourceNode (Variables|Default|GetUnitGatherer) self))

(event EventClearCommandQueue
  (Utilities|Array|Clear (Variables|Default|GetCommandQueue))
  (AI|Navigation|StopMovement (Variables|Default|GetAIController))
  (Utilities|Time|ClearandInvalidateTimerbyHandle (Variables|/Game/Blueprints/Components/UnitGatherer.UnitGatherer_C|GetGatherResourceTimer (Variables|Default|GetUnitGatherer))))

(event EventGatherCommand
  (params (TargetResource :type Actor%20Object%20Reference))
  (Default|HandleGatherCommand (Variables|Default|GetUnitGatherer) self TargetResource))

(fn ConstructionScript
  (|CallParentFunction))

(fn HandleCommandQueue
  (params (CommandQueue :type Array%20of%20F%20Unit%20Command%20Structures))
  (if (Utilities|Array|IsNotEmpty CommandQueue)
    (bind _output_get (LocalVariables|SetCurrentCommand (Utilities|Array|Get(acopy) CommandQueue)))
    (switch Utilities|FlowControl|Switch|SwitchonEUnitCommand (.commandtype _output_get)
      (:NewEnumerator0
        (CallFunction|HandleMoveCommandinQueue (Variables|Default|GetCommandQueue) (LocalVariables|GetCurrentCommand) (Variables|Default|GetUnitMovement) self (Variables|Default|GetAIController)))
      (:NewEnumerator1
        (CallFunction|HandleAttackCommandinQueue (Variables|Default|GetCommandQueue) (LocalVariables|GetCurrentCommand) (Variables|Default|GetUnitCombat) self (Variables|Default|GetAIController)))
      (:NewEnumerator4
        (CallFunction|HandleGatherCommandinQueue (Variables|Default|GetCommandQueue) (LocalVariables|GetCurrentCommand) (Variables|Default|GetUnitGatherer) self))
      (:NewEnumerator5
        (CallFunction|HandleDropOffCommandinQueue (Variables|Default|GetCommandQueue) (LocalVariables|GetCurrentCommand) (Variables|Default|GetUnitGatherer) self)))))

(fn GetUnitCommandQueue
  (return))