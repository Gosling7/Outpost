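; Base enemy unit that autonomously hunts, chases and attacks the nearest BP_BaseCharacter within aggro range.
; Looping timers chain the search, move and attack phases, falling back when the target is lost or out of range.
; AI MoveTo uses an offset navmesh point, with pathfinding and wider-projection fallbacks.
; HealthComponent handles damage and health bar; interface messages track targeting, so death notifies attackers before destroying the actor.
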(event OnDeath(HealthComponent)
  (Development|PrintString "Enemy Unit DIED!")
  (for _array_element (Variables|Default|GetTargetedByActors)
    (Class|BPIDamageable|RemoveUnitfromEnemyTarget(Message) _array_element))
  (Actor|DestroyActor))

(event Custom|AttackTarget
  ;[0.15 0.15 0.15 0.5] Attack target
  (bind _returnvalue (Utilities|Time|SetTimerbyEvent (delegate Custom|TryAttack) (Variables|Combat|GetAttackSpeedInSec) true))
  (Variables|Default|SetAttackTargetTimer _returnvalue))

(event Custom|LookFor
  ;[0.15 0.15 0.15 0.5] Look for target
  (Utilities|LookforTargetMacro
    (:Found
      (Utilities|Time|ClearandInvalidateTimerbyHandle (Variables|Default|GetLookForTargetToAttackTimer))
      (Class|BPIDamageable|AddEnemytoTargetedbyActors(Message) (Variables|Combat|GetTargetActor) self)
      (CallFunction|MovetoTarget))))

(event Custom|LookForTarget
  ;[0.15 0.15 0.15 0.5] Look for target
  (bind _returnvalue (Utilities|Time|SetTimerbyEvent (delegate Custom|LookFor) (Variables|Combat|GetLookForTargetRefreshTime) true))
  (Variables|Default|SetLookForTargetToAttackTimer _returnvalue))

(event Custom|TryAttack
  ;[0.15 0.15 0.15 0.5] Attack target
  (Variables|Combat|GetTargetActor
    (:then
      (if (Utilities|CheckIsTargetinRange)
        (bind _returnvalue (Game|Damage|ApplyDamage (Variables|Combat|GetTargetActor) (Variables|Combat|GetDamage) (AI|GetAIController self) 0))
        (Development|PrintString (Utilities|String|Append "Applied: " (Utilities|String|ToString(Float) _returnvalue) " damage"))
        (else
          (Utilities|Time|ClearandInvalidateTimerbyHandle (Variables|Default|GetAttackTargetTimer))
          (CallFunction|MovetoTarget))))
    (:else
      (Utilities|Time|ClearandInvalidateTimerbyHandle (Variables|Default|GetAttackTargetTimer))
      (CallFunction|LookforTarget))))

(event Custom|TryMove
  ;[0.15 0.15 0.15 0.5] Move to target
  (Variables|Combat|GetTargetActor
    (:then
      (Utilities|Time|ClearandInvalidateTimerbyHandle (Variables|Default|GetMoveToTargetTimer))
      (bind _validlocation (CallFunction|FindValidLocation "0, 0, 0" (Variables|Combat|GetTargetActor)))
      (AI|AIMoveTo self _validlocation (Variables|Combat|GetTargetActor) (Variables|Navigation|GetAcceptance%20Radius) true
        (:OnSuccess
          (CallFunction|AttackTarget))))
    (:else
      (Utilities|Time|ClearandInvalidateTimerbyHandle (Variables|Default|GetMoveToTargetTimer))
      (CallFunction|LookforTarget))))

(event Custom|MoveToTarget
  ;[0.15 0.15 0.15 0.5] Move to target
  (bind _returnvalue (Utilities|Time|SetTimerbyEvent (delegate Custom|TryMove) (Variables|Combat|GetMoveToTargetRefreshTime) true))
  (Variables|Default|SetMoveToTargetTimer _returnvalue))

(event EventBeginPlay
  ;[0.15 0.15 0.15 0.5] BeginPlay
  (Utilities|FlowControl|Sequence
    (:then_0
      (bind _output_get (Variables|Default|SetHealthBar (UserInterface|GetWidget (Variables|Default|GetHealthBarWidget))))
      (Default|SetupHealthBar (Variables|Default|GetHealthComponent) _output_get))
    (:then_1
      (CallFunction|LookforTarget))))

(event EventRemoveUnitfromEnemyTarget
  (Variables|Combat|SetTargetActor 0)
  (Utilities|Time|ClearandInvalidateTimerbyHandle (Variables|Combat|GetApplyDamageTimer))
  (Utilities|Time|ClearandInvalidateTimerbyHandle (Variables|Combat|GetMoveToUnitTimer))
  (CallFunction|LookforTarget))

(event EventAddEnemytoTargetedbyActors
  (params (EnemyActor :type Actor%20Object%20Reference))
  (Utilities|Array|AddUnique (Variables|Default|GetTargetedByActors) EnemyActor))

(event Game|Damage|EventAnyDamage
  (params (Damage :type Float%20%28single-precision%29) (DamageType :type Damage%20Type%20Object%20Reference) (InstigatedBy :type Controller%20Object%20Reference) (DamageCauser :type Actor%20Object%20Reference))
  (Default|TakeDamage (Variables|Default|GetHealthComponent) Damage (Variables|Default|GetHealthBar))
  (Development|PrintString (Utilities|String|Append "Enemy has taken: " (Utilities|String|ToString(Float) Damage) " damage")))

(fn ConstructionScript)

(fn FindValidLocation
  (params (TargetLocation :type Vector :default "0, 0, 0") (TargetActor :type Actor%20Object%20Reference))
  (Utilities|IsValid TargetActor
    (:Is%20Valid
      (Variables|Default|SetTargetLocation (Transformation|GetActorLocation TargetActor))
      (Variables|Default|SetDirectionToTarget (Class|KismetMathLibrary|VectorNormal2D (- (Variables|Default|GetTargetLocation) (Transformation|GetActorLocation)) 0.0001))
      (bind _output_get (Variables|Default|SetPreferredTargetLocation (- (Variables|Default|GetTargetLocation) (* (Variables|Default|GetDirectionToTarget) (Variables|Navigation|GetDirectionToTargetDistanceOffset) 0.5))))
      (bind _output_get_2 (Variables|Default|SetNearestValidPoint (.ProjectedLocation (AI|Navigation|ProjectPointtoNavigation (Class|NavigationSystemV1|GetNavigationSystem) _output_get 0 0 (Math|Conversions|ToVector(Float) (Variables|Navigation|GetValidPointSearchRadius))))))
      (if (.ReturnValue (AI|Navigation|ProjectPointtoNavigation (Class|NavigationSystemV1|GetNavigationSystem) _output_get 0 0 (Math|Conversions|ToVector(Float) (Variables|Navigation|GetValidPointSearchRadius))))
        (return _output_get_2)
        (else
          (bind _returnvalue (Class|NavigationSystemV1|FindPathtoLocationSynchronously (Transformation|GetActorLocation) (Variables|Default|GetTargetLocation) 0 0))
          (if (Utilities|IsValid _returnvalue)
            (bind _output_get_3 (Variables|Default|SetFinalPathPoint (Utilities|Array|Get(acopy) (Variables|/Script/NavigationSystem.NavigationPath|GetPathPoints _returnvalue) (Utilities|Array|LastIndex (Variables|/Script/NavigationSystem.NavigationPath|GetPathPoints _returnvalue)))))
            (return _output_get_3)
            (else
              (bind _output_get_4 (Variables|Default|SetExpandedTargetLocation (+ (* (Variables|Default|GetDirectionToTarget) (Variables|Navigation|GetDirectionToTargetDistanceOffset)) (Variables|Default|GetTargetLocation))))
              (bind _output_get_5 (Variables|Default|SetNearestValidPoint (.ProjectedLocation (AI|Navigation|ProjectPointtoNavigation _output_get_4 0 0 (Math|Conversions|ToVector(Float) (* (Variables|Navigation|GetValidPointSearchRadius) (Variables|Navigation|GetValidPointSearchRadiusMultiplier)))))))
              (if (.ReturnValue (AI|Navigation|ProjectPointtoNavigation _output_get_4 0 0 (Math|Conversions|ToVector(Float) (* (Variables|Navigation|GetValidPointSearchRadius) (Variables|Navigation|GetValidPointSearchRadiusMultiplier)))))
                (return _output_get_5)
                (else
                  (Development|PrintString "All navigation attempts failed. Worker cannot reach the tree!" true true "(R=1.000000,G=0.000000,B=0.000000,A=1.000000)"))))))))
    (:Is%20Not%20Valid
      (return TargetLocation))))

(fn GetIsAttackMoveCommand
  (return false))

(fn GetResourceCount
  (return 0))

(fn GetSelectedUnits
  (return 0))

(fn GrabSelectedUnits
  (return 0))