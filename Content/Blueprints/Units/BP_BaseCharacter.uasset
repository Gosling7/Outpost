(event OnDeath(HealthComponent)
  (Development|PrintString "Friendly Unit DIED!")
  (for _array_element (Variables|Combat|GetTargetedByActors)
    (Class|BIDamageable|RemoveUnitfromEnemyTarget(Message) _array_element))
  (Actor|DestroyActor))

(event OnDamageTaken(HealthComponent)
  (Development|PrintString (Utilities|String|Append "Current Friendly Unit Health: " (Utilities|String|ToString(Float) (Variables|/Game/Blueprints/Components/HealthComponent.HealthComponent_C|GetHealth (Variables|Default|GetHealthComponent))))))

(event Custom|CustomEvent
  (params (Location :type Vector))
  (bind (_x _y) (Math|Vector|BreakVector Location))
  (bind _acceptance_radius (Variables|Navigation|GetAcceptance%20Radius))
  ;[0.15 0.15 0.15 0.5] Stary Movement EventUnitMoveCommand()
  (AI|Navigation|StopMovement (AI|GetAIController self))
  (Rendering|Debug|DrawDebugSphere (Math|Vector|MakeVector _x _y 0.0) _acceptance_radius 12 "(R=0.172437,G=0.000000,B=1.000000,A=1.000000)" 3.0)
  (AI|AIMoveTo (AI|GetAIController self) (Math|Vector|MakeVector _x _y 0.0) 0 _acceptance_radius "Default" "Enable" true true))

(event EventBeginPlay
  ;[0.15 0.15 0.15 0.5] Setup Selected Unit Widget
  (Variables|Default|SetAIController (AI|GetAIController self))
  (Variables|Default|SetRTSController (Game|GetPlayerController 0))
  (bind _returnvalue (UserInterface|CreateWidget "/Game/Blueprints/Widgets/WBP_SelectedUnit.WBP_SelectedUnit_C"))
  (bind _output_get (Variables|Default|SetSelectedUnitWidget _returnvalue))
  (Variables|/Game/Blueprints/Widgets/WBP_SelectedUnit.WBP_SelectedUnit_C|SetUnitReferance _output_get self)
  (Appearance|SetBrushfromTexture (Variables|/Game/Blueprints/Widgets/WBP_SelectedUnit.WBP_SelectedUnit_C|GetUnitImage _returnvalue) (Variables|Default|Get2DImage) false)
  (bind _output_get_2 (Variables|Default|SetHealthBar (UserInterface|GetWidget (Variables|Default|GetHealthBarWidget))))
  (Default|SetupHealthBar (Variables|Default|GetHealthComponent) _output_get_2))

(event EventAddEnemytoTargetedbyActors
  (params (EnemyActor :type Actor%20Object%20Reference))
  (Utilities|Array|AddUnique (Variables|Combat|GetTargetedByActors) EnemyActor))

(event EventSetSelected
  (params (Value :type Boolean))
  (bind _selectordecal (Variables|Default|GetSelectorDecal))
  (if Value
    (Rendering|SetVisibility _selectordecal true false)
    (else
      (Rendering|SetVisibility _selectordecal false false))))

(event EventUnitMoveCommand
  (params (TargetLocation :type Vector :default "0, 0, 0") (TargetActor :type Actor%20Object%20Reference) (SelectedUnitCount :type Integer) (UnitIndex :type Integer) (LocationCenterOfSelectedUnits :type Vector :default "0, 0, 0") (ForwardVectorOfSelectedUnits :type Vector :default "0, 0, 0"))
  (Variables|Default|SetSelected%20Unit%20Count 0)
  (Variables|Formation|SetUnit%20Index 0)
  (Variables|Formation|SetCenterLocation "0, 0, 0")
  (AI|Navigation|StopMovement (Variables|Default|GetAIController))
  (bind _validlocation (CallFunction|FindValidLocation TargetLocation TargetActor))
  (if (> 0 1)
    (Variables|Default|SetTargetLocation _validlocation)
    (else
      (AI|AIMoveTo (Variables|Default|GetAIController) _validlocation 0 (Variables|Navigation|GetAcceptance%20Radius) "Default" "Default" true true))))

(event EventSelectThis
  ;[0.15 0.15 0.15 0.5] Selection
  (Rendering|SetVisibility (Variables|Default|GetSelectorDecal) true false)
  (Class|BIRTS|AddUnittoSelectedUnitsArea(Message) (Game|GetPlayerController 0) (Variables|Default|GetSelectedUnitWidget)))

(event EventDeselectThis
  ;[0.15 0.15 0.15 0.5] Selection
  (Rendering|SetVisibility (Variables|Default|GetSelectorDecal) false false)
  (Widget|RemovefromParent (Variables|Default|GetSelectedUnitWidget)))

(event EventHighlightUnit
  ;[0.15 0.15 0.15 0.5] Highlight
  (Rendering|Components|Decal|SetDecalMaterial (Variables|Default|GetSelectorDecal) "/Game/Materials/M_HighlightDecal.M_HighlightDecal"))

(event EventUnHighlightUnit
  ;[0.15 0.15 0.15 0.5] Highlight
  (Rendering|Components|Decal|SetDecalMaterial (Variables|Default|GetSelectorDecal) "/Game/Materials/M_SelectorDecal.M_SelectorDecal"))

(event Game|Damage|EventAnyDamage
  (params (Damage :type Float%20%28single-precision%29) (DamageType :type Damage%20Type%20Object%20Reference) (InstigatedBy :type Controller%20Object%20Reference) (DamageCauser :type Actor%20Object%20Reference))
  (Default|TakeDamage (Variables|Default|GetHealthComponent) Damage (Variables|Default|GetHealthBar))
  (Development|PrintString (Utilities|String|Append "Taken: " (Utilities|String|ToString(Float) Damage) " damage")))

(fn ConstructionScript)

(fn FindValidLocation
  (params (TargetLocation :type Vector :default "0, 0, 0") (TargetActor :type Actor%20Object%20Reference))
  (Utilities|IsValid TargetActor
    (:Is%20Valid
      (Variables|Default|SetTargetLocation (Transformation|GetActorLocation TargetActor))
      (Variables|Default|SetDirectionToTarget (Class|KismetMathLibrary|VectorNormal2D (- (Variables|Default|GetTargetLocation) (Transformation|GetActorLocation)) 0.0001))
      (bind _output_get (Variables|Default|SetPreferredTargetLocation (- (Variables|Default|GetTargetLocation) (* (Variables|Default|GetDirectionToTarget) (Variables|Navigation|GetDirectionToTargetDistanceOffset) 0.5))))
      (bind _output_get_2 (Variables|Default|SetNearestValidPoint (.ProjectedLocation (AI|Navigation|ProjectPointtoNavigation (Class|NavigationSystemV1|GetNavigationSystem) _output_get 0 0 (Math|Conversions|ToVector(Float) (Variables|Navigation|GetValidPointSearchRadius))))))
      (if (.ReturnValue (AI|Navigation|ProjectPointtoNavigation (Class|NavigationSystemV1|GetNavigationSystem) _output_get 0 0 (Math|Conversions|ToVector(Float) (Variables|Navigation|GetValidPointSearchRadius))))
        (return _output_get_2)
        (else
          (bind _returnvalue (Class|NavigationSystemV1|FindPathtoLocationSynchronously (Transformation|GetActorLocation) (Variables|Default|GetTargetLocation) 0 0))
          (if (Utilities|IsValid _returnvalue)
            (bind _output_get_3 (Variables|Default|SetFinalPathPoint (Utilities|Array|Get(acopy) (Variables|/Script/NavigationSystem.NavigationPath|GetPathPoints _returnvalue) (Utilities|Array|LastIndex (Variables|/Script/NavigationSystem.NavigationPath|GetPathPoints _returnvalue)))))
            (return _output_get_3)
            (else
              (bind _output_get_4 (Variables|Default|SetExpandedTargetLocation (+ (* (Variables|Default|GetDirectionToTarget) (Variables|Navigation|GetDirectionToTargetDistanceOffset)) (Variables|Default|GetTargetLocation))))
              (bind _output_get_5 (Variables|Default|SetNearestValidPoint (.ProjectedLocation (AI|Navigation|ProjectPointtoNavigation _output_get_4 0 0 (Math|Conversions|ToVector(Float) (* (Variables|Navigation|GetValidPointSearchRadius) (Variables|Navigation|GetValidPointSearchRadiusMultiplier)))))))
              (if (.ReturnValue (AI|Navigation|ProjectPointtoNavigation _output_get_4 0 0 (Math|Conversions|ToVector(Float) (* (Variables|Navigation|GetValidPointSearchRadius) (Variables|Navigation|GetValidPointSearchRadiusMultiplier)))))
                (return _output_get_5)
                (else
                  (Development|PrintString "All navigation attempts failed. Worker cannot reach the tree!" true true "(R=1.000000,G=0.000000,B=0.000000,A=1.000000)"))))))))
    (:Is%20Not%20Valid
      (return TargetLocation))))

(fn GetIsAttackMoveCommand
  (return false))

(fn GetIsNodeDepleted
  (return false))

(fn GetIsNodeGatherable
  (return false))

(fn GetResourceCount
  (return 0))

(fn GetResourceLeft
  (return 0))

(fn GrabSelectedUnits
  (return 0))