(event OnGatherCommand(StateMachineComponent)
  (bind _statemachinecomponent (Variables|Default|GetStateMachineComponent))
  (Utilities|Array|RemoveItem (Variables|/Game/Blueprints/Components/StateMachineComponent.StateMachineComponent_C|GetCommandQueue _statemachinecomponent) (Variables|/Game/Blueprints/Components/StateMachineComponent.StateMachineComponent_C|GetCurrentCommand _statemachinecomponent))
  (Default|SetState (Variables|Default|GetStateMachineComponent) "NewEnumerator3"))

(event OnBuildCommand(StateMachineComponent)
  (bind _statemachinecomponent (Variables|Default|GetStateMachineComponent))
  (Utilities|Array|RemoveItem (Variables|/Game/Blueprints/Components/StateMachineComponent.StateMachineComponent_C|GetCommandQueue _statemachinecomponent) (Variables|/Game/Blueprints/Components/StateMachineComponent.StateMachineComponent_C|GetCurrentCommand _statemachinecomponent))
  (Class|BIBuilding|AddtoActiveBuilders(Message) (Variables|Default|GetBuildingToBuild) self)
  (Class|BIBuilding|Build(Message) (Variables|Default|GetBuildingToBuild)))

(event Custom|Gather
  ;[0.15 0.15 0.15 0.5] Gather Action
  (if (Variables|Default|GetbCarriesMaxResources)
    (CallFunction|Dropoff)
    (else
      (AI|Navigation|StopMovement (Variables|Default|GetAIController))
      (Utilities|IsValid (Variables|Default|GetResourceNode)
        (:Is%20Valid
          (bind _validlocation (CallFunction|FindValidLocationtoNavigate "0, 0, 0" (Variables|Default|GetResourceNode)))
          (AI|AIMoveTo (Variables|Default|GetAIController) _validlocation 0 (Variables|Default|GetAcceptance%20Radius) "Default" "Default" true true
            (:OnMoveFinished
              (bind _returnvalue (Utilities|Time|SetTimerbyEvent (delegate Custom|OnGatherTick) 1.0 true))
              (Variables|Default|SetResourceCollectTimer _returnvalue))))
        (:Is%20Not%20Valid
          (Utilities|Time|ClearandInvalidateTimerbyHandle (Variables|Default|GetResourceCollectTimer))
          (CallFunction|FindNewResourceNode))))))

(event Custom|OnGatherTick
  ;[0.15 0.15 0.15 0.5] Gather Action
  (Transformation|SetRelativeRotation (Variables|Default|GetAxe) (Math|Rotator|MakeRotator 0.0 0.0 0.0) false false)
  (Utilities|IsValid (Variables|Default|GetResourceNode)
    (:Is%20Valid
      (if (>= (Variables|Gathering|GetCarriedResourceCount) (Variables|Gathering|GetMaxCarriedResourceCount))
        (Variables|Default|SetbCarriesMaxResources true)
        (Variables|Default|SetResourceCollectTimer "")
        (CallFunction|Dropoff)
        (elif (== (Utilities|GetClass (Variables|Default|GetResourceNode)) "/Game/Blueprints/ResourceNodes/BP_RN_Tree.BP_RN_Tree_C")
          (Variables|Gathering|SetCarriedResourceType "NewEnumerator0")
          (Utilities|FlowControl|Sequence
            (:then_0
              (bind _swingtrack (Timeline|AxeSwing PlayFromStart)
                (:Update
                  (Transformation|SetRelativeRotation (Variables|Default|GetAxe) (Math|Rotator|MakeRotator 0.0 (* _swingtrack -9e+01) 0.0) false false))))
            (:then_1
              (Variables|Gathering|SetCarriedResourceCount (+ (Variables|Gathering|GetCarriedResourceCount) (Variables|Default|GetResourceCountPerGatherTick)) :!label _label)
              (bind _value (Class|BIResourceNode|GetIsNodeGatherable(Message) (Variables|Default|GetResourceNode)))
              (if _value
                (Class|BIResourceNode|DecreaseResourcesLeft(Message) (Variables|Default|GetResourceNode) (Variables|Default|GetResourceCountPerGatherTick))
                (if (>= (Variables|Gathering|GetCarriedResourceCount) (Variables|Gathering|GetMaxCarriedResourceCount))
                  (Variables|Default|SetbCarriesMaxResources true)
                  (bind _value_2 (Class|BIResourceNode|GetIsNodeGatherable(Message) (Variables|Default|GetResourceNode)))
                  (if (not _value_2)
                    (Utilities|Time|ClearandInvalidateTimerbyHandle (Variables|Default|GetResourceCollectTimer))
                    (Class|BIResourceNode|ResourceNodeDepleted(Message) (Variables|Default|GetResourceNode))
                    (CallFunction|Gather)))
                (else
                  (Class|BIResourceNode|ResourceNodeDepleted(Message) (Variables|Default|GetResourceNode))
                  (Utilities|Time|ClearandInvalidateTimerbyHandle (Variables|Default|GetResourceCollectTimer))
                  (CallFunction|FindNewResourceNode)))))
          (elif (== (Utilities|GetClass (Variables|Default|GetResourceNode)) "/Game/Blueprints/ResourceNodes/BP_RN_BerryBush.BP_RN_BerryBush_C")
            (Variables|Gathering|SetCarriedResourceType "NewEnumerator1")
            (goto _label)))))
    (:Is%20Not%20Valid
      (Utilities|Time|ClearandInvalidateTimerbyHandle (Variables|Default|GetResourceCollectTimer))
      (CallFunction|FindNewResourceNode))))

(event Custom|FindNewResourceNode
  (bind _returnvalue (Transformation|GetActorLocation))
  (bind _returnvalue_2 (Transformation|GetActorLocation))
  ;[0.15 0.15 0.15 0.5] Find New Resource Node
  (Utilities|Array|Clear (Variables|Gathering|GetDetectedNearbyResourceNodes))
  (switch Utilities|FlowControl|Switch|SwitchonEResourceType (Variables|Gathering|GetCarriedResourceType)
    (:NewEnumerator0
      (bind (_outhits _returnvalue_3) (Collision|MultiSphereTraceForObjects _returnvalue _returnvalue 1e+03 (Utilities|Array|MakeArray "ObjectTypeQuery8") false 0 "None" true "(R=1.000000,G=0.000000,B=0.000000,A=1.000000)" "(R=0.000000,G=1.000000,B=0.000000,A=1.000000)" 3.0))
      (Variables|Gathering|SetResourceNodesTraceSphereHits _outhits)
      (if _returnvalue_3
        (for _array_element (Variables|Gathering|GetResourceNodesTraceSphereHits) :!label _label
          (Utilities|Array|AddUnique (Variables|Gathering|GetDetectedNearbyResourceNodes) (.HitActor (Collision|BreakHitResult _array_element))))
        (Variables|Default|SetResourceNode (.ReturnValue (Actor|FindNearestActor (Transformation|GetActorLocation) (Variables|Gathering|GetDetectedNearbyResourceNodes))))
        (CallFunction|Gather)))
    (:NewEnumerator1
      (bind (_outhits_2 _returnvalue_4) (Collision|MultiSphereTraceForObjects _returnvalue_2 _returnvalue_2 1e+03 (Utilities|Array|MakeArray "ObjectTypeQuery7") false 0 "None" true "(R=1.000000,G=0.000000,B=0.000000,A=1.000000)" "(R=0.000000,G=1.000000,B=0.000000,A=1.000000)" 3.0))
      (Variables|Gathering|SetResourceNodesTraceSphereHits _outhits_2)
      (if _returnvalue_4
        (goto _label)))))

(event Custom|ExecuteBuildCommand
  ;[0.15 0.15 0.15 0.5] Stare (chyba do wywalenia)
  (Utilities|Array|RemoveItem (Variables|Default|GetCommandQueue) (Variables|Default|GetCurrentCommand))
  (Class|BIBuilding|AddtoActiveBuilders(Message) (Variables|Default|GetBuildingToBuild) self)
  (Class|BIBuilding|Build(Message) (Variables|Default|GetBuildingToBuild)))

(event EventDropoff
  ;[0.15 0.15 0.15 0.5] Dropoff Action
  (switch Utilities|FlowControl|Switch|SwitchonEResourceType (Variables|Gathering|GetCarriedResourceType)
    (:NewEnumerator0
      (bind _outactors (Actor|GetAllActorsOfClass "/Game/Blueprints/Buildings/BP_B_LumberCamp.BP_B_LumberCamp_C"))
      (Variables|Gathering|SetDropoffBuilding (.ReturnValue (Actor|FindNearestActor (Transformation|GetActorLocation) _outactors))))
    (:NewEnumerator1
      (bind _outactors_2 (Actor|GetAllActorsOfClass "/Game/Blueprints/Buildings/BP_B_Granary.BP_B_Granary_C"))
      (Variables|Gathering|SetDropoffBuilding (.ReturnValue (Actor|FindNearestActor (Transformation|GetActorLocation) _outactors_2)))))
  (bind _validlocation (CallFunction|FindValidLocationtoNavigate "0, 0, 0" (Variables|Gathering|GetDropoffBuilding)))
  (AI|AIMoveTo (Variables|Default|GetAIController) _validlocation 0 (Variables|Default|GetAcceptance%20Radius) "Default" "Default" true true
    (:OnMoveFinished
      (Class|BIResourceManager|IncreasePlayerResources(Message) (Game|GetPlayerState 0) (Utilities|Struct|MakeF_Resource (Variables|Gathering|GetCarriedResourceType) (Variables|Gathering|GetCarriedResourceCount)))
      (Variables|Gathering|SetCarriedResourceCount 0)
      (Variables|Default|SetbCarriesMaxResources false)
      (if (Variables|Default|GetbIsWorking)
        (Utilities|IsValid (Variables|Default|GetResourceNode)
          (:Is%20Valid
            (CallFunction|Gather))
          (:Is%20Not%20Valid
            (Utilities|Time|ClearandInvalidateTimerbyHandle (Variables|Default|GetResourceCollectTimer))
            (CallFunction|FindNewResourceNode)))))))

(event EventBuildCommand
  (params (TargetActor :type BP%20B%20Base%20Object%20Reference))
  ;[0.15 0.15 0.15 0.5] Build Command
  (Variables|Default|SetBuildingToBuild TargetActor)
  (Rendering|Debug|DrawDebugSphere (Math|Vector|MakeVector (.x (+ (Transformation|GetActorLocation (Variables|Default|GetBuildingToBuild)) (* 3e+02 (Math|Vector|Normalize (- (Transformation|GetActorLocation) (Transformation|GetActorLocation (Variables|Default|GetBuildingToBuild))))))) (.y (+ (Transformation|GetActorLocation (Variables|Default|GetBuildingToBuild)) (* 3e+02 (Math|Vector|Normalize (- (Transformation|GetActorLocation) (Transformation|GetActorLocation (Variables|Default|GetBuildingToBuild))))))) 0.0) 1e+02 12 "(R=1.000000,G=1.000000,B=1.000000,A=1.000000)" 5.0)
  (Utilities|Array|Add (Variables|/Game/Blueprints/Components/StateMachineComponent.StateMachineComponent_C|GetCommandQueue (Variables|Default|GetStateMachineComponent)) (Utilities|Struct|MakeF_UnitCommand "NewEnumerator0" (Math|Vector|MakeVector (.x (+ (Transformation|GetActorLocation (Variables|Default|GetBuildingToBuild)) (* 3e+02 (Math|Vector|Normalize (- (Transformation|GetActorLocation) (Transformation|GetActorLocation (Variables|Default|GetBuildingToBuild))))))) (.y (+ (Transformation|GetActorLocation (Variables|Default|GetBuildingToBuild)) (* 3e+02 (Math|Vector|Normalize (- (Transformation|GetActorLocation) (Transformation|GetActorLocation (Variables|Default|GetBuildingToBuild))))))) 0.0) 0))
  (Utilities|Array|Add (Variables|/Game/Blueprints/Components/StateMachineComponent.StateMachineComponent_C|GetCommandQueue (Variables|Default|GetStateMachineComponent)) (Utilities|Struct|MakeF_UnitCommand "NewEnumerator3" "0.000000,0.000000,0.000000" (Variables|Default|GetTargetActor)))
  (Default|TryProcessNextCommandState (Variables|Default|GetStateMachineComponent)))

(event EventUnitMoveCommand
  (params (TargetLocation :type Vector :default "0, 0, 0") (TargetActor :type Actor%20Object%20Reference) (SelectedUnitCount :type Integer) (UnitIndex :type Integer) (LocationCenterOfSelectedUnits :type Vector :default "0, 0, 0") (ForwardVectorOfSelectedUnits :type Vector :default "0, 0, 0"))
  ;[0.15 0.15 0.15 0.5] Move Command
  (Variables|Default|SetbIsWorking false)
  (Variables|Default|SetResourceCollectTimer "")
  (Class|BIResourceNode|RemovefromActiveWorkers(Message) (Variables|Default|GetResourceNode) self)
  (AI|Navigation|StopMovement (Variables|Default|GetAIController))
  (bind _validlocation (CallFunction|FindValidLocationtoNavigate TargetLocation TargetActor))
  (AI|AIMoveTo (Variables|Default|GetAIController) _validlocation 0 (Variables|Default|GetAcceptance%20Radius) "Default" "Default" true true))

(event EventSetNotWorking
  (Variables|Default|SetbIsWorking false)
  (Utilities|Time|ClearandInvalidateTimerbyHandle (Variables|Default|GetResourceCollectTimer))
  (Class|BIResourceNode|RemovefromActiveWorkers(Message) (Variables|Default|GetResourceNode) self)
  (Variables|Default|SetResourceNode 0))

(event EventGatherCommand
  (params (TargetResource :type Actor%20Object%20Reference))
  ;[0.15 0.15 0.15 0.5] Gather Command
  (Variables|Default|SetResourceNode TargetResource)
  (Variables|Default|SetbIsWorking true) ; Sprawdzić kiedy dokładnie ustawiać tę flagę
  (Class|BIResourceNode|AddtoActiveWorkers(Message) (Variables|Default|GetResourceNode) self)
  (if (Variables|Default|GetbCarriesMaxResources)
    (CallFunction|Dropoff)
    (else
      (CallFunction|Gather))))

(fn ConstructionScript
  (|CallParentFunction))