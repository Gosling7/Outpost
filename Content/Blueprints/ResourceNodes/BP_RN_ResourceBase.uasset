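; Base Blueprint for a gatherable resource node that holds a finite resource count and tracks the workers active on it.
; Construction fills the count to its maximum, events set or decrease it, and getters report the amount, depleted and gatherable states.
; Workers register uniquely; the depletion event, not triggered within this file, removes them while iterating the same array, then destroys the node.
; UnitGatherCommand is an empty stub.
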(event EventResourceNodeDepleted
  (for _array_element (Variables|Default|GetActiveWorkers)
    (CallFunction|RemovefromActiveWorkers _array_element))
  (Actor|DestroyActor))

(event EventAddtoActiveWorkers
  (params (Worker :type Actor%20Object%20Reference))
  (Utilities|Array|AddUnique (Variables|Default|GetActiveWorkers) Worker))

(event EventRemovefromActiveWorkers
  (params (Worker :type Actor%20Object%20Reference))
  (Utilities|Array|RemoveItem (Variables|Default|GetActiveWorkers) Worker))

(event EventDecreaseResourcesLeft
  (params (ResourceCount :type Integer))
  (Variables|Default|SetResourcesLeft (- (Variables|Default|GetResourcesLeft) ResourceCount)))

(event EventSetResourceLeft
  (params (ResourceCount :type Integer))
  (Variables|Default|SetResourcesLeft ResourceCount))

(fn ConstructionScript
  (Variables|Default|SetResourcesLeft (Variables|Default|GetResourcesMax)))

(fn GetIsNodeDepleted
  (return (<= (Variables|Default|GetResourcesLeft) 0)))

(fn GetIsNodeGatherable
  (return (> (Variables|Default|GetResourcesLeft) 0)))

(fn GetResourceLeft
  (return (Variables|Default|GetResourcesLeft)))

(fn UnitGatherCommand
  (params (TargetResource :type Actor%20Object%20Reference)))