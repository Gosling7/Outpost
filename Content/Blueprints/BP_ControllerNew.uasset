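; RTS player controller that handles camera edge scrolling, unit selection and right-click orders, and creates the building menu and resources widgets.
; A screen-edge macro offsets the camera pawn when the cursor nears viewport borders.
; Selection-box input goes to the HUD outside building mode, with release always forwarded.
; Right-click traces under the cursor and messages HUD-selected units to attack enemies, gather resources or move, spawning cursor FX for moves.
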(event Input|EnhancedActionEvents|EnhancedInputActionIA_SelectionBox
  (params (ActionValue :type Boolean) (ElapsedSeconds :type Float%20%28double-precision%29) (TriggeredSeconds :type Float%20%28double-precision%29) (InputAction :type Input%20Action%20Object%20Reference :default "/Game/Input/IA_SelectionBox.IA_SelectionBox"))
  ;[0.15 0.15 0.15 0.5 30] Selection Box
  (:Started
    (if (not (Variables|Default|GetbIsInBuildingMode))
      (Class|BIHUD|LeftButtonPressed(Message) (Variables|Default|GetHUD) (.HitLocation (CallFunction|GetHitUnderCursor)))))
  (:Ongoing
    (if (not (Variables|Default|GetbIsInBuildingMode))
      (Class|BIHUD|LeftButtonHeld(Message) (Variables|Default|GetHUD))))
  (:Canceled
    (Class|BIHUD|LeftButtonReleased(Message) (Variables|Default|GetHUD) :!label _label))
  (:Completed
    (goto _label)))

(event Input|EnhancedActionEvents|EnhancedInputActionIA_RightClick
  (params (ActionValue :type Boolean) (ElapsedSeconds :type Float%20%28double-precision%29) (TriggeredSeconds :type Float%20%28double-precision%29) (InputAction :type Input%20Action%20Object%20Reference :default "/Game/Input/IA_RightClick.IA_RightClick"))
  (:Completed
    (CallFunction|HandleRightClick)))

(event EventBeginPlay
  ;[0.15 0.15 0.15 0.5 30] BeginPlay
  (bind _asbp_camera_pawn (Utilities|Casting|CastToBP_CameraPawn (Game|Player|GetPlayerPawn 0)))
  (Variables|Default|SetCameraPawn _asbp_camera_pawn)
  (Input|SetInputModeGameandUI self 0 "LockAlways" false false)
  (Input|AddMappingContext (PlayerController|LocalPlayerSubsystems|GetEnhancedInputLocalPlayerSubsystem) "/Game/Input/IMC_RTS.IMC_RTS" 0 "(bIgnoreAllPressedKeysUntilRelease=True,bForceImmediately=False,bNotifyUserSettings=False)")
  (Variables|Default|SetHUD (HUD|GetHUD))
  (CallFunction|AddWidgets))

(event Input|MouseEvents|MouseX
  (params (AxisValue :type Float%20%28single-precision%29))
  ;[0.15 0.15 0.15 0.5 30] Screen Edge Movement
  (bind (_delta_x_speed _delta_y_speed) (Utilities|ScreenEdgeMovement)
    (:returnNode
      (Transformation|AddActorLocalOffset (Variables|Default|GetCameraPawn) (Math|Vector|MakeVector _delta_x_speed _delta_y_speed 0.0) false false))))

(event Input|MouseEvents|MouseY
  (params (AxisValue :type Float%20%28single-precision%29))
  ;[0.15 0.15 0.15 0.5 30] Screen Edge Movement
  (Utilities|ScreenEdgeMovement) ; enters at Mouse y
)

(fn ConstructionScript)

(fn AddWidgets
  (bind _returnvalue (UserInterface|CreateWidget "/Game/Blueprints/Widgets/WBP_BuildingMenu.WBP_BuildingMenu_C"))
  (bind _output_get (Variables|Default|SetBuildingMenuWidget _returnvalue))
  (Widget|SetVisibility _output_get "Hidden")
  (bind _returnvalue_2 (UserInterface|CreateWidget "/Game/Blueprints/Widgets/WBP_Resources.WBP_Resources_C"))
  (bind _output_get_2 (Variables|Default|SetResourcesWidget _returnvalue_2))
  (UserInterface|Viewport|AddtoViewport _output_get_2 0))

(fn GetHitUnderCursor
  (bind _hitresult (Game|Player|GetHitResultUnderCursorbyChannel "TraceTypeQuery1" true))
  (bind (_bblockinghit _binitialoverlap _time _distance _location _impactpoint _normal _impactnormal _physmat _hitactor) (Collision|BreakHitResult _hitresult))
  (return _bblockinghit _location _hitactor))

(fn IssueMoveCommand
  (params (SelectedUnits :type Array%20of%20Actor%20Object%20References) (TargetLocation :type Vector) (TargetActor :type Actor%20Object%20Reference))
  (for _array_element SelectedUnits
    (Class|BIPlayerUnit|MoveCommand(Message) _array_element TargetLocation TargetActor))
  (CallFunction|SpawnMovePartciles TargetLocation))

(fn SpawnMovePartciles
  (params (TargetLocation :type Vector))
  (Niagara|SpawnSystematLocation "/Game/Cursor/FX_Cursor.FX_Cursor" TargetLocation))

(fn HandleRightClick
  (bind _hitresult (Game|Player|GetHitResultUnderCursorbyChannel "TraceTypeQuery1" true))
  (bind (_bblockinghit _binitialoverlap _time _distance _location _impactpoint _normal _impactnormal _physmat _hitactor) (Collision|BreakHitResult _hitresult))
  (LocalVariables|SetRightClickedLocation _location)
  (LocalVariables|SetRightClickedActor _hitactor)
  (if (Utilities|ClassIsChildOf (Utilities|GetClass _hitactor) "/Game/Blueprints/Units/BP_EnemyCharacter.BP_EnemyCharacter_C")
    (bind _units (Class|BIHUD|GetSelectedUnits(Message) (Variables|Default|GetHUD)))
    (CallFunction|IssueAttackCommand _units (LocalVariables|GetRightClickedActor) (LocalVariables|GetRightClickedLocation))
    (elif (Utilities|ClassIsChildOf (Utilities|GetClass _hitactor) "/Game/Blueprints/ResourceNodes/BP_RN_ResourceBase.BP_RN_ResourceBase_C")
      (bind _units_2 (Class|BIHUD|GetSelectedUnits(Message) (Variables|Default|GetHUD)))
      (CallFunction|IssueGatherCommand _units_2 (LocalVariables|GetRightClickedActor) (LocalVariables|GetRightClickedLocation))
      (else
        (bind _units_3 (Class|BIHUD|GetSelectedUnits(Message) (Variables|Default|GetHUD)))
        (CallFunction|IssueMoveCommand _units_3 (LocalVariables|GetRightClickedLocation))))))

(fn IssueAttackCommand
  (params (SelectedUnits :type Array%20of%20Actor%20Object%20References) (AttackTarget :type Actor%20Object%20Reference) (TargetLocation :type Vector))
  (for _array_element SelectedUnits
    (Class|BIPlayerUnit|AttackCommand(Message) _array_element AttackTarget TargetLocation)))

(fn IssueGatherCommand
  (params (SelectedUnits :type Array%20of%20Actor%20Object%20References) (TargetResource :type Actor%20Object%20Reference) (TargetLocation :type Vector))
  (for _array_element SelectedUnits
    (Class|BIGathererUnit|GatherCommand(Message) _array_element TargetResource)))