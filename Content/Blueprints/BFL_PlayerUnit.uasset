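; Blueprint function library for player units that handles queued unit commands and finds navigable destinations.
; Move, attack, gather and drop-off handlers remove the command from the queue, then pass execution to the matching movement, combat or gatherer component.
; FindValidLocationToNavigate projects a point short of the target actor onto the navmesh, falling back to a path's end point, then a wider search beyond it.
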(fn HandleMoveCommandinQueue
  (params (CommandQueue :type Array%20of%20F%20Unit%20Command%20Structures) (CurrentCommand :type F%20Unit%20Command%20Structure) (UnitMovementComponent :type Unit%20Movement%20Object%20Reference) (PlayerUnit :type Actor%20Object%20Reference) (AIController :type AI%20Controller%20Object%20Reference))
  (bind (_commandtype _targetlocation _targetactor) (Utilities|Struct|BreakF_UnitCommand CurrentCommand))
  (Utilities|Array|RemoveItem CommandQueue CurrentCommand)
  (Default|ExecuteMoveCommand UnitMovementComponent AIController _targetlocation _targetactor PlayerUnit))

(fn HandleAttackCommandinQueue
  (params (CommandQueue :type Array%20of%20F%20Unit%20Command%20Structures) (CurrentCommand :type F%20Unit%20Command%20Structure) (UnitCombatComponent :type Unit%20Combat%20Object%20Reference) (PlayerUnit :type Actor%20Object%20Reference) (AIController :type AI%20Controller%20Object%20Reference))
  (Utilities|Array|RemoveItem CommandQueue CurrentCommand)
  (Default|ExecuteAttackCommand UnitCombatComponent PlayerUnit AIController CurrentCommand))

(fn HandleGatherCommandinQueue
  (params (CommandQueue :type Array%20of%20F%20Unit%20Command%20Structures) (CurrentCommand :type F%20Unit%20Command%20Structure) (UnitGathererComponent :type Unit%20Gatherer%20Object%20Reference) (PlayerUnit :type Actor%20Object%20Reference))
  (Utilities|Array|RemoveItem CommandQueue CurrentCommand)
  (Default|ExecuteGatherCommand UnitGathererComponent PlayerUnit))

(fn FindValidLocationtoNavigate
  (params (PlayerUnit :type Actor%20Object%20Reference) (TargetLocation :type Vector) (TargetActor :type Actor%20Object%20Reference))
  (LocalVariables|SetUnit PlayerUnit)
  (Utilities|IsValid TargetActor
    (:Is%20Valid
      (LocalVariables|SetlocationToNavigate (Transformation|GetActorLocation TargetActor))
      (LocalVariables|SetDirectionToTarget (Class|KismetMathLibrary|VectorNormal2D (- (LocalVariables|GetlocationToNavigate) (Transformation|GetActorLocation (LocalVariables|GetUnit))) 0.0001))
      (bind _output_get (LocalVariables|SetPreferredTargetLocation (- (LocalVariables|GetlocationToNavigate) (* (LocalVariables|GetDirectionToTarget) (LocalVariables|GetDirectionToTargetDistanceOffset) 0.5))))
      (bind _output_get_2 (LocalVariables|SetNearestValidPoint (.ProjectedLocation (AI|Navigation|ProjectPointtoNavigation (Class|NavigationSystemV1|GetNavigationSystem) 0 _output_get 0 0 (Math|Conversions|ToVector(Float) (LocalVariables|GetValidPointSearchRadius))))))
      (if (.ReturnValue (AI|Navigation|ProjectPointtoNavigation (Class|NavigationSystemV1|GetNavigationSystem) 0 _output_get 0 0 (Math|Conversions|ToVector(Float) (LocalVariables|GetValidPointSearchRadius))))
        (return _output_get_2)
        (else
          (bind _returnvalue (Class|NavigationSystemV1|FindPathtoLocationSynchronously 0 (Transformation|GetActorLocation (LocalVariables|GetUnit)) (LocalVariables|GetlocationToNavigate) 0 0))
          (if (Utilities|IsValid _returnvalue)
            (bind _output_get_3 (LocalVariables|SetFinalPathPoint (Utilities|Array|Get(acopy) (Variables|/Script/NavigationSystem.NavigationPath|GetPathPoints _returnvalue) (Utilities|Array|LastIndex (Variables|/Script/NavigationSystem.NavigationPath|GetPathPoints _returnvalue)))))
            (return _output_get_3)
            (else
              (bind _output_get_4 (LocalVariables|SetExpandedTargetLocation (+ (* (LocalVariables|GetDirectionToTarget) (LocalVariables|GetDirectionToTargetDistanceOffset)) (LocalVariables|GetlocationToNavigate))))
              (bind _output_get_5 (LocalVariables|SetNearestValidPoint (.ProjectedLocation (AI|Navigation|ProjectPointtoNavigation 0 _output_get_4 0 0 (Math|Conversions|ToVector(Float) (* (LocalVariables|GetValidPointSearchRadius) (LocalVariables|GetValidPointSearchRadiusMultiplier)))))))
              (if (.ReturnValue (AI|Navigation|ProjectPointtoNavigation 0 _output_get_4 0 0 (Math|Conversions|ToVector(Float) (* (LocalVariables|GetValidPointSearchRadius) (LocalVariables|GetValidPointSearchRadiusMultiplier)))))
                (return _output_get_5)
                (else
                  (Development|PrintString 0 "All navigation attempts failed. Worker cannot reach the tree!" true true "(R=1.000000,G=0.000000,B=0.000000,A=1.000000)"))))))))
    (:Is%20Not%20Valid
      (return TargetLocation))))

(fn HandleDropOffCommandinQueue
  (params (CommandQueue :type Array%20of%20F%20Unit%20Command%20Structures) (CurrentCommand :type F%20Unit%20Command%20Structure) (UnitGathererComponent :type Unit%20Gatherer%20Object%20Reference) (PlayerUnit :type Actor%20Object%20Reference))
  (Utilities|Array|RemoveItem CommandQueue CurrentCommand)
  (Default|ExecuteDropOffCommand UnitGathererComponent PlayerUnit))