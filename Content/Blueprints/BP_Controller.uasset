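; RTS player controller that sets up HUD widgets, edge-scrolls the camera pawn and turns mouse input into unit and building commands.
; Right-click sends gather, attack, attack-move or move orders to the HUD's selected units, spreading groups over concentric formation rings.
; Building mode shows grid-snapped previews, including L-shaped wall paths respawned each tick.
; Placement checks and deducts player-state resources, then sends selected workers to build.
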(event Input|EnhancedActionEvents|EnhancedInputActionIA_SelectionBox
  (params (ActionValue :type Boolean) (ElapsedSeconds :type Float%20%28double-precision%29) (TriggeredSeconds :type Float%20%28double-precision%29) (InputAction :type Input%20Action%20Object%20Reference :default "/Game/Input/IA_SelectionBox.IA_SelectionBox"))
  ;[0.15 0.15 0.15 0.5 30] Selection Box
  (:Started
    (if (not (Variables|Default|GetbIsInBuildingMode))
      (Class|BIHUD|LeftButtonPressed(Message) (Variables|Default|GetHUD) (.Location (Collision|BreakHitResult (.HitResult (Game|Player|GetHitResultUnderCursorbyChannel "TraceTypeQuery1" true)))))))
  (:Ongoing
    (if (not (Variables|Default|GetbIsInBuildingMode))
      (Class|BIHUD|LeftButtonHeld(Message) (Variables|Default|GetHUD))))
  (:Canceled
    (Class|BIHUD|LeftButtonReleased(Message) (Variables|Default|GetHUD) :!label _label))
  (:Completed
    (goto _label)))

(event Input|EnhancedActionEvents|EnhancedInputActionIA_PlaceBuilding
  (params (ActionValue :type Boolean) (ElapsedSeconds :type Float%20%28double-precision%29) (TriggeredSeconds :type Float%20%28double-precision%29) (InputAction :type Input%20Action%20Object%20Reference :default "/Game/Input/IA_PlaceBuilding.IA_PlaceBuilding"))
  ;[0.15 0.15 0.15 0.5] Place Building
  (:Completed
    (if (Variables|Default|GetbIsInBuildingMode)
      (if (Utilities|IsValidClass (Variables|Default|GetSelectedBuildingClass))
        (bind _value (Class|BIResourceManager|HasEnoughResources(Message) (Game|GetPlayerState 0) (Variables|/Game/Blueprints/Buildings/BP_B_Base.BP_B_Base_C|GetCost (Variables|Default|GetBuildingToBuild))))
        (if _value
          (bind _workers (Class|BIHUD|GetSelectedWorkers(Message) (Variables|Default|GetHUD)))
          (if (and (Utilities|Array|IsNotEmpty _workers) (Variables|Default|GetbIsInBuildingMode))
            (Variables|Default|SetSelectedWorkers _workers)
            (bind _returnvalue (Game|SpawnActorfromClass (Variables|Default|GetSelectedBuildingClass) (Math|Transform|MakeTransform (Variables|Default|GetPreviewLocation) "0, 0, 0" "1.000000,1.000000,1.000000") "AlwaysSpawn" "MultiplyWithRoot" 0 0))
            (Variables|Default|SetBuildingToBuild _returnvalue)
            (Class|BIResourceManager|DecreasePlayerResources(Message) (Game|GetPlayerState 0) (Variables|/Game/Blueprints/Buildings/BP_B_Base.BP_B_Base_C|GetCost (Variables|Default|GetBuildingToBuild)))
            (bind _returnvalue_2 (Rendering|Material|CreateDynamicMaterialInstance "/Engine/VREditor/UI/FrameMaterial.FrameMaterial" "None" "None" :!class /Script/Engine.KismetMaterialLibrary))
            (Rendering|Material|SetMaterial (Variables|/Game/Blueprints/Buildings/BP_B_Base.BP_B_Base_C|GetBuildingMesh (Variables|Default|GetBuildingToBuild)) 0 _returnvalue_2)
            (Collision|SetActorEnableCollision (Variables|Default|GetBuildingToBuild) false)
            (for _array_element (Variables|Default|GetSelectedWorkers)
              (Class|BIWorkerUnit|BuildCommand(Message) _array_element (Variables|Default|GetBuildingToBuild)))
            (Utilities|Array|Clear (Variables|Default|GetSelectedWorkers))))))))

(event Input|EnhancedActionEvents|EnhancedInputActionIA_RightClick
  (params (ActionValue :type Boolean) (ElapsedSeconds :type Float%20%28double-precision%29) (TriggeredSeconds :type Float%20%28double-precision%29) (InputAction :type Input%20Action%20Object%20Reference :default "/Game/Input/IA_RightClick.IA_RightClick"))
  (bind _currentpreview (Variables|Default|GetCurrentPreview))
  ;[0.15 0.15 0.15 0.5 30] Right Mouse Button
  (:Completed
    (if (Variables|Default|GetbIsInBuildingMode)
      ;;[0.15 0.15 0.15 0.5] Reset Placement
      (Variables|Default|SetbIsInWallPreview false)
      (Variables|Default|SetbIsInBuildingMode false)
      (CallFunction|DestroyPreviewWalls (Variables|Default|GetPreviewArray))
      (Utilities|IsValid _currentpreview
        (:Is%20Valid
          (Actor|DestroyActor _currentpreview)))
      (else
        (bind _output_get (Variables|Default|SetCursorHitResult (.HitResult (Game|Player|GetHitResultUnderCursorbyChannel "TraceTypeQuery1" true))))
        (if (Class|KismetSystemLibrary|DoesClassImplementInterface (Utilities|GetClass (.HitActor (Collision|BreakHitResult _output_get))) "/Game/Blueprints/Interfaces/BI_ResourceNode.BI_ResourceNode_C")
          (bind _units (Class|BIHUD|GetSelectedUnits(Message) (Variables|Default|GetHUD)))
          (for _array_element _units
            (if (Utilities|DoesObjectImplementInterface _array_element "/Game/Blueprints/Interfaces/BI_WorkerUnit.BI_WorkerUnit_C")
              (Class|BIWorkerUnit|GatherCommand(Message) _array_element (.HitActor (Collision|BreakHitResult (Variables|Default|GetCursorHitResult))))))
          (elif (Utilities|ClassIsChildOf (Utilities|GetClass (.HitActor (Collision|BreakHitResult _output_get))) "/Game/Blueprints/Units/BP_BaseEnemyCharacter.BP_BaseEnemyCharacter_C")
            (bind _units_2 (Class|BIHUD|GetSelectedUnits(Message) (Variables|Default|GetHUD)))
            (for _array_element_2 _units_2
              (if (Utilities|DoesObjectImplementInterface _array_element_2 "/Game/Blueprints/Interfaces/BI_PlayerUnit.BI_PlayerUnit_C")
                (Class|BIPlayerUnit|AttackCommand(Message) _array_element_2 (.HitActor (Collision|BreakHitResult (Variables|Default|GetCursorHitResult))))))
            (else
              ;;[0.15 0.15 0.15 0.5] Sprawdzic czy klikniety budynek jest w trakcie budowy
              (if (Utilities|ClassIsChildOf (Utilities|GetClass (.HitActor (Collision|BreakHitResult (Variables|Default|GetCursorHitResult)))) "/Game/Blueprints/Buildings/BP_B_Base.BP_B_Base_C")
                _
                (else
                  _))
              (if (Variables|Default|GetbIsAttackMoveIssued)
                (bind _units_3 (Class|BIHUD|GetSelectedUnits(Message) (Variables|Default|GetHUD)))
                (for _array_element_3 _units_3
                  (if (Utilities|DoesObjectImplementInterface _array_element_3 "/Game/Blueprints/Interfaces/BI_PlayerUnit.BI_PlayerUnit_C")
                    (Class|BIPlayerUnit|AttackMoveCommand(Message) _array_element_3 (.Location (Collision|BreakHitResult (Variables|Default|GetCursorHitResult))))))
                (Variables|Default|SetbIsAttackMoveIssued false)
                (Development|PrintString "AttackMove Issued!")
                (else
                  (bind _units_4 (Class|BIHUD|GetSelectedUnits(Message) (Variables|Default|GetHUD)))
                  (Variables|Default|SetSelectedUnits _units_4)
                  (Variables|Default|SetSelectedUnitsCount (Utilities|Array|Length _units_4))
                  (Variables|Default|SetRemainingSelectedUnits (Variables|Default|GetSelectedUnitsCount))
                  (Variables|Default|SetRightClickLocation (.Location (Collision|BreakHitResult (Variables|Default|GetCursorHitResult))))
                  (if (> (Utilities|Array|Length (Variables|Default|GetSelectedUnits)) 1)
                    (Utilities|FlowControl|Sequence
                      (:then_0
                        (CallFunction|FormFormationRings (.Location (Collision|BreakHitResult (Variables|Default|GetCursorHitResult))) (Variables|Default|GetSelectedUnitsCount)))
                      (:then_1
                        (for _array_element_4 (Variables|Default|GetFormationRings)
                          (for (_array_element_5 _array_index) (.UnitPositions (Utilities|Struct|BreakF_FormationRing _array_element_4))
                            (bind _output_get_2 (Variables|Default|SetArray%20Element _array_element_5))
                            (bind _output_get_3 (Variables|Default|SetArray%20Index _array_index))
                            (bind _output_get_4 (Variables|Default|SetNewVar (Utilities|Array|Get(acopy) (Variables|Default|GetSelectedUnits) _output_get_3)))
                            (Class|BIPlayerUnit|MoveCommand(Message) _output_get_4 _output_get_2)))
                        (Niagara|SpawnSystematLocation "/Game/Cursor/FX_Cursor.FX_Cursor" (Variables|Default|GetRightClickLocation))))
                    (else
                      (for _array_element_6 (Variables|Default|GetSelectedUnits)
                        (Class|BIPlayerUnit|MoveCommand(Message) _array_element_6 (Variables|Default|GetRightClickLocation)))
                      (Niagara|SpawnSystematLocation "/Game/Cursor/FX_Cursor.FX_Cursor" (Variables|Default|GetRightClickLocation)))))))))))))

(event EventBeginPlay
  ;[0.15 0.15 0.15 0.5 30] BeginPlay()
  (bind _asbp_camera_pawn (Utilities|Casting|CastToBP_CameraPawn (Game|Player|GetPlayerPawn 0)))
  (Variables|Default|SetCameraPawnRefference _asbp_camera_pawn)
  (Input|SetInputModeGameandUI self 0 "LockAlways" false false)
  (Input|AddMappingContext (PlayerController|LocalPlayerSubsystems|GetEnhancedInputLocalPlayerSubsystem) "/Game/Input/IMC_RTS.IMC_RTS" 0 "(bIgnoreAllPressedKeysUntilRelease=True,bForceImmediately=False,bNotifyUserSettings=False)")
  (Variables|Default|SetHUD (HUD|GetHUD))
  (bind _returnvalue (UserInterface|CreateWidget "/Game/Blueprints/Widgets/WBP_BuildingMenu.WBP_BuildingMenu_C"))
  (bind _output_get (Variables|Default|SetBuildingMenuWidget _returnvalue))
  (Widget|SetVisibility _output_get "Hidden")
  (UserInterface|Viewport|AddtoViewport (Variables|Default|GetBuildingMenuWidget) 0)
  (bind _returnvalue_2 (UserInterface|CreateWidget "/Game/Blueprints/Widgets/WBP_SelectedUnitsArea.WBP_SelectedUnitsArea_C"))
  (Variables|Default|SetSelectedUnitsArea _returnvalue_2)
  (UserInterface|Viewport|AddtoViewport _returnvalue_2 0)
  (bind _returnvalue_3 (UserInterface|CreateWidget "/Game/Blueprints/Widgets/WBP_Resources.WBP_Resources_C"))
  (bind _output_get_2 (Variables|Default|SetResourcesWidget _returnvalue_3))
  (UserInterface|Viewport|AddtoViewport _output_get_2 0))

(event EventSelectBuilding
  (params (BuildingClass :type BP%20B%20Base%20Class%20Reference))
  ;[0.15 0.15 0.15 0.5] Building Menu
  (Variables|Default|SetbIsInBuildingMode true)
  (Variables|Default|SetbIsInWallPreview false)
  (if (Utilities|IsValid (Variables|Default|GetCurrentPreview))
    (CallFunction|DestroyPreviewWalls (Variables|Default|GetPreviewArray))
    (Actor|DestroyActor (Variables|Default|GetCurrentPreview)))
  (bind _output_get (Variables|Default|SetSelectedBuildingClass BuildingClass))
  (bind _returnvalue (Game|SpawnActorfromClass _output_get (Math|Transform|MakeTransform "0, 0, 0" "0, 0, 0" "1.000000,1.000000,1.000000") "Undefined" "MultiplyWithRoot" 0 0))
  (Collision|SetActorEnableCollision _returnvalue false)
  (bind _output_get_2 (Variables|Default|SetCurrentPreview _returnvalue))
  (bind _returnvalue_2 (Rendering|Material|CreateDynamicMaterialInstance "/Engine/VREditor/UI/FrameMaterial.FrameMaterial" "None" "None" :!class /Script/Engine.KismetMaterialLibrary))
  (Rendering|Material|SetMaterial (Actor|GetComponentbyClass _output_get_2 "/Script/Engine.StaticMeshComponent") 0 _returnvalue_2)
  (Transformation|SetActorLocation (Math|Vector|MakeVector 0.0 0.0 -5e+01) false false))

(event EventTick
  (params (DeltaSeconds :type Float%20%28single-precision%29))
  (bind _currentpreview (Variables|Default|GetCurrentPreview))
  ;[0.15 0.15 0.15 0.5] Monitor Preview Building Positon
  (if (Utilities|IsValid (Variables|Default|GetCurrentPreview))
    (if (Actor|ActorHasTag (Variables|Default|GetCurrentPreview) "Building")
      (bind _newparam (CallFunction|SnapBuildings (Variables|Default|GetCurrentPreview)))
      (Variables|Default|SetPreviewLocation _newparam)
      (Transformation|SetActorLocation (Variables|Default|GetCurrentPreview) (Math|Vector|MakeVector (.x (Variables|Default|GetPreviewLocation)) (.y (Variables|Default|GetPreviewLocation)) 0.0) false false)
      (elif (Actor|ActorHasTag _currentpreview "Wall")
        (Rendering|SetActorHiddenInGame _currentpreview true)
        (bind _newparam_2 (CallFunction|SnapWalls))
        (Variables|Default|SetPreviewLocation _newparam_2)
        (if (Variables|Default|GetbIsInWallPreview)
          (bind _newparam_3 (CallFunction|SnapWalls))
          (bind _transform (CallFunction|FindGridPath (Variables|Default|GetWallStartLocation) _newparam_3))
          (bind _output_get (Variables|Default|SetWallGridPath _transform))
          (CallFunction|DestroyPreviewWalls (Variables|Default|GetPreviewArray))
          (CallFunction|SpawnPreviewWalls _output_get))))))

(event EventAddUnittoSelectedUnitsArea
  (params (SelectedUnitWidget :type User%20Widget%20Object%20Reference))
  (Class|HorizontalBox|AddChildtoHorizontalBox (Variables|/Game/Blueprints/Widgets/WBP_SelectedUnitsArea.WBP_SelectedUnitsArea_C|GetUnitsBox (Variables|Default|GetSelectedUnitsArea)) SelectedUnitWidget))

(event Input|MouseEvents|MouseX
  (params (AxisValue :type Float%20%28single-precision%29))
  ;[0.15 0.15 0.15 0.5 30] Screen Edge Movement
  (bind (_delta_x_speed _delta_y_speed) (Utilities|ScreenEdgeMovement)
    (:returnNode
      (Transformation|AddActorLocalOffset (Variables|Default|GetCameraPawnRefference) (Math|Vector|MakeVector _delta_x_speed _delta_y_speed 0.0) false false))))

(event Input|MouseEvents|MouseY
  (params (AxisValue :type Float%20%28single-precision%29))
  ;[0.15 0.15 0.15 0.5 30] Screen Edge Movement
  (Utilities|ScreenEdgeMovement) ; enters at Mouse y
)

(event Input|KeyboardEvents|A
  (params (Key :type Key%20Structure :default "None"))
  ;[0.15 0.15 0.15 0.5 30] Enter Attack Move
  (:Pressed
    (Variables|Default|SetbIsAttackMoveIssued true)
    (Development|PrintString "AttackMove activated.")))

(fn ConstructionScript)

(fn FormFormationRings
  (params (RightClickLocation :type Vector) (SelectedUnitsCount :type Integer))
  (Variables|Default|SetRemainingSelectedUnits SelectedUnitsCount)
  (LocalVariables|SetrightClickPosition RightClickLocation)
  (while (> (Variables|Default|GetRemainingSelectedUnits) 0)
    (LocalVariables|SetringRadius (+ (Variables|Default|GetBaseRingRadius) (* (LocalVariables|GetformationRingCount) (Variables|Default|GetRingSpacing))))
    (LocalVariables|SetunitsInRing (Math|Float|Floor (/ (* (* (Math|Trig|GetPI) 2.0) (LocalVariables|GetringRadius)) (Variables|Default|GetUnitSpacing))))
    (if (> (LocalVariables|GetunitsInRing) (Variables|Default|GetRemainingSelectedUnits))
      (LocalVariables|SetunitsInRing (Math|Integer|Min(Integer) (LocalVariables|GetunitsInRing) (Variables|Default|GetRemainingSelectedUnits))))
    (Variables|Default|SetRemainingSelectedUnits (- (Variables|Default|GetRemainingSelectedUnits) (LocalVariables|GetunitsInRing)))
    (Math|Integer|IncrementInt (LocalVariables|GetformationRingCount)
      (:%20%20
        (for _index (range 0 (- (LocalVariables|GetunitsInRing) 1))
          (bind _output_get (LocalVariables|Setradians (* (* (/ _index (LocalVariables|GetunitsInRing)) 360) (/ (Math|Trig|GetPI) 1.8e+02))))
          (LocalVariables|SetpositionX (* (Math|Trig|Cos(Radians) _output_get) (LocalVariables|GetringRadius)))
          (LocalVariables|SetpositionY (* (Math|Trig|Sin(Radians) (LocalVariables|Getradians)) (LocalVariables|GetringRadius)))
          (bind _output_get_2 (LocalVariables|SetunitPosition (+ (LocalVariables|GetrightClickPosition) (Math|Vector|MakeVector (LocalVariables|GetpositionX) (LocalVariables|GetpositionY) 0.0))))
          (Utilities|Array|Add (LocalVariables|GetunitPositions) _output_get_2))
        (Utilities|Array|Add (Variables|Default|GetFormationRings) (Utilities|Struct|MakeF_FormationRing (LocalVariables|GetringRadius) (LocalVariables|GetunitsInRing) (LocalVariables|GetunitPositions)))))))

(fn GetLocationUnderCursor
  (bind _hitresult (Game|Player|GetHitResultUnderCursorbyChannel "TraceTypeQuery1" true))
  (bind (_bblockinghit _binitialoverlap _time _distance _location) (Collision|BreakHitResult _hitresult))
  (return _bblockinghit _location))

(fn SnapWalls
  (bind _location (CallFunction|GetLocationUnderCursor))
  (return (Math|Vector|MakeVector (Math|Conversions|ToFloat(Integer) (+ (* (Math|Float|Floor (/ (.x _location) (Variables|Default|GetGridSize))) (Variables|Default|GetGridSize)) (/ (Variables|Default|GetGridSize) 2))) (Math|Conversions|ToFloat(Integer) (+ (* (Math|Float|Floor (/ (.y _location) (Variables|Default|GetGridSize))) (Variables|Default|GetGridSize)) (/ (Variables|Default|GetGridSize) 2))) (.z _location))))

(fn SnapBuildings
  (params (Building :type Actor%20Object%20Reference))
  (bind _location (CallFunction|GetLocationUnderCursor))
  (bind _location_2 (CallFunction|GetLocationUnderCursor))
  (if (Actor|ActorHasTag Building "3x3")
    ;[0.15 0.15 0.15 0.5] Grid Size jest dodatkowo dzielony przez 2, aby budynek zajmujący nieparzysty wymiar w inny sposób się snapował - jest przesunięty odpowiednio o połowę komórki gridu
    (return (Math|Vector|MakeVector (Math|Conversions|ToFloat(Integer) (+ (* (Math|Float|Round (/ (.x _location) (Variables|Default|GetGridSize))) (Variables|Default|GetGridSize)) (/ (Variables|Default|GetGridSize) 2))) (Math|Conversions|ToFloat(Integer) (+ (* (Math|Float|Round (/ (.y _location) (Variables|Default|GetGridSize))) (Variables|Default|GetGridSize)) (/ (Variables|Default|GetGridSize) 2))) (.z _location)))
    (else
      ;[0.15 0.15 0.15 0.5] Snapowanie dla budynków zajmujących parzysty wymiar - czyli to "normalne"/początkowe snapowanie.
      (return (Math|Vector|MakeVector (Math|Conversions|ToFloat(Integer) (* (Math|Float|Round (/ (.x _location_2) (Variables|Default|GetGridSize))) (Variables|Default|GetGridSize))) (Math|Conversions|ToFloat(Integer) (* (Math|Float|Round (/ (.y _location_2) (Variables|Default|GetGridSize))) (Variables|Default|GetGridSize))) (.z _location_2))))))

(fn FindGridPath
  (params (Start :type Vector) (End :type Vector))
  (LocalVariables|SetCurrentWallPosition Start)
  (LocalVariables|SetWallEndLocation End)
  (while (!= (.x (LocalVariables|GetCurrentWallPosition)) (.x (LocalVariables|GetWallEndLocation)))
    (if (> (.x (LocalVariables|GetCurrentWallPosition)) (.x (LocalVariables|GetWallEndLocation)))
      (bind _output_get (LocalVariables|SetCurrentWallPosition (Math|Vector|MakeVector (- (.x (LocalVariables|GetCurrentWallPosition)) (Variables|Default|GetGridSize)) (.y (LocalVariables|GetCurrentWallPosition)) 0.0)))
      (LocalVariables|SetWallTransform (+ _output_get "100.000000,0.000000,0.000000"))
      (else
        (bind _output_get_2 (LocalVariables|SetCurrentWallPosition (Math|Vector|MakeVector (+ (.x (LocalVariables|GetCurrentWallPosition)) (Variables|Default|GetGridSize)) (.y (LocalVariables|GetCurrentWallPosition)) 0.0)))
        (LocalVariables|SetWallTransform (- _output_get_2 "100.000000,0.000000,0.000000"))))
    (LocalVariables|SetWallRotation "0, 0, 0")
    (Utilities|Array|Add (LocalVariables|GetTransforms%20to%20pass) (Math|Transform|MakeTransform (LocalVariables|GetWallTransform) (LocalVariables|GetWallRotation) "1.000000,1.000000,1.000000")))
  (while (!= (.y (LocalVariables|GetCurrentWallPosition)) (.y (LocalVariables|GetWallEndLocation)))
    (if (> (.y (LocalVariables|GetCurrentWallPosition)) (.y (LocalVariables|GetWallEndLocation)))
      (bind _output_get_3 (LocalVariables|SetCurrentWallPosition (Math|Vector|MakeVector (.x (LocalVariables|GetCurrentWallPosition)) (- (.y (LocalVariables|GetCurrentWallPosition)) (Variables|Default|GetGridSize)) 0.0)))
      (LocalVariables|SetWallTransform (+ _output_get_3 "0.000000,100.000000,0.000000"))
      (else
        (bind _output_get_4 (LocalVariables|SetCurrentWallPosition (Math|Vector|MakeVector (.x (LocalVariables|GetCurrentWallPosition)) (+ (.y (LocalVariables|GetCurrentWallPosition)) (Variables|Default|GetGridSize)) 0.0)))
        (LocalVariables|SetWallTransform (- _output_get_4 "0.000000,100.000000,0.000000"))))
    (LocalVariables|SetWallRotation "0.000000,90.000000,0.000000")
    (Utilities|Array|Add (LocalVariables|GetTransforms%20to%20pass) (Math|Transform|MakeTransform (LocalVariables|GetWallTransform) (LocalVariables|GetWallRotation) "1.000000,1.000000,1.000000")))
  (return (LocalVariables|GetTransforms%20to%20pass)))

(fn SpawnPreviewWalls
  (params (Path :type Array%20of%20Transforms))
  (for _array_element Path
    (bind _returnvalue (Game|SpawnActorfromClass "/Game/Blueprints/Buildings/BP_B_Wall.BP_B_Wall_C" (Math|Transform|MakeTransform (.location _array_element) (.rotation _array_element) "1.000000,1.000000,1.000000") "Undefined" "MultiplyWithRoot" 0 0))
    (Rendering|Material|SetMaterial (Variables|/Game/Blueprints/Buildings/BP_B_Wall.BP_B_Wall_C|GetCube _returnvalue) 0 "/Engine/VREditor/UI/FrameMaterial.FrameMaterial")
    (Utilities|Array|Add (Variables|Default|GetPreviewArray) _returnvalue)))

(fn DestroyPreviewWalls
  (params (PreviewArray :type Array%20of%20BP%20B%20Wall%20Object%20References))
  (for _array_element PreviewArray
    (Actor|DestroyActor _array_element))
  (Utilities|Array|Clear PreviewArray))

(fn FindValidLocationtoNavigate
  (params (TargetLocation :type Vector :default "0, 0, 0") (TargetActor :type Actor%20Object%20Reference))
  (return "0, 0, 0"))

(fn GetActiveBuilders
  (return 0))

(fn GetIsAttackMoveCommand
  (return false))

(fn GetResourceCount
  (return 0))

(fn GrabSelectedUnits
  (return 0))