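; Unit component that runs an RTS-style gather loop for player units, currently handling wood from trees and drop-off at lumber camps.
; A looping timer drains the target node until carry capacity or depletion, registering the unit as an active worker.
; Movement, gathering and drop-off are queued as unit commands; drop-off credits PlayerState and resumes gathering.
; Invalid targets are replaced via sphere trace for the nearest node of the carried type.
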(event Custom|ExecuteDropOffCommand
  (params (PlayerUnit :type Actor%20Object%20Reference))
  (Utilities|FlowControl|Delay 0.5)
  (Class|BIResourceManager|IncreasePlayerResources(Message) (Game|GetPlayerState 0) (Utilities|Struct|MakeF_Resource (Variables|Default|GetCarriedResourceType) (Variables|Default|GetCarriedResources)))
  (Variables|Default|SetCarriedResources 0)
  (CallFunction|HandleGatherCommand PlayerUnit))

(event Custom|ExecuteGatherCommand
  (params (PlayerUnit :type Actor%20Object%20Reference))
  (bind _returnvalue (Utilities|Time|SetTimerbyEvent (delegate Custom|GatherResource) 0.5 true))
  (Variables|Default|SetGatherResourceTimer _returnvalue))

(event Custom|GatherResource
  (CallFunction|Gather (stale Custom|ExecuteGatherCommand PlayerUnit) (Variables|Default|GetGatherResourceTimer)))

(fn HandleGatherCommand
  (params (PlayerUnit :type Actor%20Object%20Reference) (ClickedResource :type Actor%20Object%20Reference))
  (Utilities|IsValid ClickedResource
    (:Is%20Valid
      (Variables|Default|SetTargetResource ClickedResource)
      (bind _validlocation (CallFunction|FindValidLocationtoNavigate PlayerUnit "0, 0, 0" (Variables|Default|GetTargetResource) :!label _label))
      (LocalVariables|SetTargetResourceLocation _validlocation)
      (Utilities|Array|Add (LocalVariables|GetCommands) (Utilities|Struct|MakeF_UnitCommand "NewEnumerator0" (LocalVariables|GetTargetResourceLocation) 0))
      (Utilities|Array|Add (LocalVariables|GetCommands) (Utilities|Struct|MakeF_UnitCommand "NewEnumerator4" "0.000000,0.000000,0.000000" (Variables|Default|GetTargetResource)))
      (Class|BIPlayerUnit|AddCommandstoQueue(Message) PlayerUnit (LocalVariables|GetCommands))
      (Class|BIPlayerUnit|CheckCommandQueue(Message) PlayerUnit))
    (:Is%20Not%20Valid
      (Utilities|IsValid (Variables|Default|GetTargetResource)
        (:Is%20Valid
          (goto _label))
        (:Is%20Not%20Valid
          (CallFunction|FindNewResourceNode PlayerUnit)
          (CallFunction|HandleGatherCommand PlayerUnit))))))

(fn FindNewResourceNode
  (params (PlayerUnit :type Actor%20Object%20Reference))
  (bind _returnvalue (Transformation|GetActorLocation PlayerUnit))
  (bind _returnvalue_2 (Transformation|GetActorLocation PlayerUnit))
  (Utilities|Array|Clear (LocalVariables|GetDetectedNearbyResourceNodes))
  (switch Utilities|FlowControl|Switch|SwitchonEResourceType (Variables|Default|GetCarriedResourceType)
    (:NewEnumerator0
      (bind (_outhits _returnvalue_3) (Collision|MultiSphereTraceForObjects _returnvalue _returnvalue 1e+03 (Utilities|Array|MakeArray "ObjectTypeQuery8") false 0 "None" true "(R=1.000000,G=0.000000,B=0.000000,A=1.000000)" "(R=0.000000,G=1.000000,B=0.000000,A=1.000000)" 3.0))
      (LocalVariables|SetResourceNodesTraceSphereHits _outhits)
      (if _returnvalue_3
        (for _array_element (LocalVariables|GetResourceNodesTraceSphereHits) :!label _label
          (Utilities|Array|AddUnique (LocalVariables|GetDetectedNearbyResourceNodes) (.HitActor (Collision|BreakHitResult _array_element))))
        (bind _output_get (Variables|Default|SetTargetResource (.ReturnValue (Actor|FindNearestActor (Transformation|GetActorLocation PlayerUnit) (LocalVariables|GetDetectedNearbyResourceNodes)))))))
    (:NewEnumerator1
      (bind (_outhits_2 _returnvalue_4) (Collision|MultiSphereTraceForObjects _returnvalue_2 _returnvalue_2 1e+03 (Utilities|Array|MakeArray "ObjectTypeQuery7") false 0 "None" true "(R=1.000000,G=0.000000,B=0.000000,A=1.000000)" "(R=0.000000,G=1.000000,B=0.000000,A=1.000000)" 3.0))
      (LocalVariables|SetResourceNodesTraceSphereHits _outhits_2)
      (if _returnvalue_4
        (goto _label)))))

(fn FindDropOffPoint
  (params (PlayerUnit :type Actor%20Object%20Reference))
  (bind _outactors (Actor|GetAllActorsOfClass "/Game/Blueprints/Buildings/BP_B_LumberCamp.BP_B_LumberCamp_C"))
  (Variables|Default|SetDropOffPoint (.ReturnValue (Actor|FindNearestActor (Transformation|GetActorLocation PlayerUnit) _outactors))))

(fn Gather
  (params (PlayerUnit :type Actor%20Object%20Reference) (GatherResourceTimer :type Timer%20Handle%20Structure))
  (if (>= (Variables|Default|GetCarriedResources) (Variables|Default|GetMaxCarriedResources))
    (Utilities|Time|ClearandInvalidateTimerbyHandle GatherResourceTimer)
    (Utilities|IsValid (Variables|Default|GetDropOffPoint)
      (:Is%20Valid
        _)
      (:Is%20Not%20Valid
        (CallFunction|FindDropOffPoint PlayerUnit)))
    (CallFunction|MovetoDropOffPoint PlayerUnit)
    (else
      (Utilities|IsValid (Variables|Default|GetTargetResource)
        (:Is%20Valid
          (if (Variables|Default|GetbIsAddedToActiveWorkers)
            _
            (else
              (Class|BIResourceNode|AddtoActiveWorkers(Message) (Variables|Default|GetTargetResource) PlayerUnit)
              (Variables|Default|SetbIsAddedToActiveWorkers true)))
          (if (== (Utilities|GetClass (Variables|Default|GetTargetResource)) "/Game/Blueprints/ResourceNodes/BP_RN_Tree.BP_RN_Tree_C")
            (Variables|Default|SetCarriedResourceType "NewEnumerator0")
            (Variables|Default|SetCarriedResources (+ (Variables|Default|GetCarriedResources) (Variables|Default|GetResourcesPerGatherTick)))
            (bind _value (Class|BIResourceNode|GetIsNodeGatherable(Message) (Variables|Default|GetTargetResource)))
            (if _value
              (Class|BIResourceNode|DecreaseResourcesLeft(Message) (Variables|Default|GetTargetResource) (Variables|Default|GetResourcesPerGatherTick))
              (if (>= (Variables|Default|GetCarriedResources) (Variables|Default|GetMaxCarriedResources))
                (Variables|Default|SetbCarriesMaxResources true)
                (bind _value_2 (Class|BIResourceNode|GetIsNodeGatherable(Message) (Variables|Default|GetTargetResource)))
                (if (not _value_2)
                  (Utilities|Time|ClearandInvalidateTimerbyHandle GatherResourceTimer)
                  (Class|BIResourceNode|ResourceNodeDepleted(Message) (Variables|Default|GetTargetResource))
                  (if (Variables|Default|GetbCarriesMaxResources)
                    (CallFunction|MovetoDropOffPoint PlayerUnit)
                    (else
                      (CallFunction|HandleGatherCommand PlayerUnit)))))
              (else
                (Class|BIResourceNode|ResourceNodeDepleted(Message) (Variables|Default|GetTargetResource))
                (Utilities|Time|ClearandInvalidateTimerbyHandle GatherResourceTimer)
                (CallFunction|HandleGatherCommand PlayerUnit)))))
        (:Is%20Not%20Valid
          (Utilities|Time|ClearandInvalidateTimerbyHandle GatherResourceTimer)
          (CallFunction|FindNewResourceNode PlayerUnit)
          (CallFunction|HandleGatherCommand PlayerUnit))))))

(fn MovetoDropOffPoint
  (params (PlayerUnit :type Actor%20Object%20Reference))
  (Utilities|Array|Add (LocalVariables|GetCommands) (Utilities|Struct|MakeF_UnitCommand "NewEnumerator0" "0.000000,0.000000,0.000000" (Variables|Default|GetDropOffPoint)))
  (Utilities|Array|Add (LocalVariables|GetCommands) (Utilities|Struct|MakeF_UnitCommand "NewEnumerator5" "0.000000,0.000000,0.000000" (Variables|Default|GetDropOffPoint)))
  (Class|BIPlayerUnit|AddCommandstoQueue(Message) PlayerUnit (LocalVariables|GetCommands))
  (Class|BIPlayerUnit|CheckCommandQueue(Message) PlayerUnit))