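; State machine component that gates queued Move, Attack, Build and Gather commands by the current state.
; TryProcessNextCommandState copies the front queue entry into CurrentCommand without removing it, then fires the matching command event dispatcher.
; Idle accepts every command, Moving excludes Gather, and Attacking allows only Move or Attack without checking for an empty queue.
; SetState assigns the state directly, and the event graph has no active logic.
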(event EventBeginPlay)

(event EventTick
  (params (DeltaSeconds :type Float%20%28single-precision%29)))

(fn TryProcessNextCommandState
  (switch Utilities|FlowControl|Switch|SwitchonEUnitState (Variables|Default|GetCurrentState)
    (:NewEnumerator0
      (if (Utilities|Array|IsNotEmpty (Variables|Default|GetCommandQueue))
        (bind _output_get (Variables|Default|SetCurrentCommand (Utilities|Array|Get(acopy) (Variables|Default|GetCommandQueue))))
        (switch Utilities|FlowControl|Switch|SwitchonEUnitCommand (.CommandType (Utilities|Struct|BreakF_UnitCommand _output_get))
          (:NewEnumerator0
            (Default|CallOnMoveCommand))
          (:NewEnumerator1
            (Default|CallOnAttackCommand))
          (:NewEnumerator3
            (Default|CallOnBuildCommand))
          (:NewEnumerator4
            (Default|CallOnGatherCommand)))))
    (:NewEnumerator1
      (if (Utilities|Array|IsNotEmpty (Variables|Default|GetCommandQueue))
        (bind _output_get_2 (Variables|Default|SetCurrentCommand (Utilities|Array|Get(acopy) (Variables|Default|GetCommandQueue))))
        (switch Utilities|FlowControl|Switch|SwitchonEUnitCommand (.CommandType (Utilities|Struct|BreakF_UnitCommand _output_get_2))
          (:NewEnumerator0
            (Default|CallOnMoveCommand))
          (:NewEnumerator1
            (Default|CallOnAttackCommand))
          (:NewEnumerator3
            (Default|CallOnBuildCommand)))))
    (:NewEnumerator2
      (bind _output_get_3 (Variables|Default|SetCurrentCommand (Utilities|Array|Get(acopy) (Variables|Default|GetCommandQueue))))
      (switch Utilities|FlowControl|Switch|SwitchonEUnitCommand (.CommandType (Utilities|Struct|BreakF_UnitCommand _output_get_3))
        (:NewEnumerator0
          (Default|CallOnMoveCommand))
        (:NewEnumerator1
          (Default|CallOnAttackCommand))))))

(fn SetState
  (params (NewParam :type EUnitState%20Enum :default "NewEnumerator0"))
  (Variables|Default|SetCurrentState NewParam))