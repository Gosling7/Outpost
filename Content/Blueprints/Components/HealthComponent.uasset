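; Actor component that tracks an actor's health and pushes changes to its health bar widget.
; Health starts at MaxHealth on BeginPlay, and SetupHealthBar sets the passed-in widget to full.
; TakeDamage subtracts damage, fires OnDamageTaken, sends the health fraction to the bar through an UpdateHealthBarWidget message, and fires OnDeath once health reaches zero or below.
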(event EventBeginPlay
  (Variables|Default|SetHealth (Variables|Default|GetMaxHealth)))

(event EventTick
  (params (DeltaSeconds :type Float%20%28single-precision%29)))

(fn TakeDamage
  (params (Damage :type Float%20%28double-precision%29) (HealthBar :type Widget%20Object%20Reference))
  (Variables|Default|SetHealth (- (Variables|Default|GetHealth) Damage))
  (Default|CallOnDamageTaken)
  (bind _output_get (LocalVariables|SethealthPercentage (/ (Variables|Default|GetHealth) (Variables|Default|GetMaxHealth))))
  (Class|BPIHUD|UpdateHealthBarWidget(Message) HealthBar _output_get)
  (if (<= (Variables|Default|GetHealth) 0.0)
    (Default|CallOnDeath)))

(fn SetupHealthBar
  (params (HealthBarWidget :type Widget%20Object%20Reference))
  (Class|BPIHUD|UpdateHealthBarWidget(Message) HealthBarWidget 1.0))