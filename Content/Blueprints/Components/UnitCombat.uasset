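; Unit combat component that carries out attack commands for player units in a command-queue-driven game.
; ExecuteAttackCommand stores the target and starts a looping attack-speed timer that applies damage while the target is in range.
; An out-of-range target stops the timer and queues move and attack commands through unit messages.
; HandleAttackCommand queues an attack or sends a move by range; attack-move resume logic is left unconnected.
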(event Custom|ExecuteAttackCommand
  (params (PlayerUnit :type Actor%20Object%20Reference) (AIController :type AI%20Controller%20Object%20Reference) (CurrentCommand :type F%20Unit%20Command%20Structure))
  (Development|PrintString "Enemy Clicked To Attack")
  (Utilities|FlowControl|Sequence
    (:then_0
      (Variables|Default|SetCurrent%20Command CurrentCommand)
      (Variables|Default|SetAIController AIController)
      (Variables|Default|SetPlayer%20Unit PlayerUnit)
      (Variables|Default|SetTargetActor (.targetactor (Variables|Default|GetCurrent%20Command)))
      (Variables|Default|SetTargetLocation (.targetlocation (Variables|Default|GetCurrent%20Command))))
    (:then_1
      (Class|BIPlayerUnit|ClearCommandQueue(Message) (Variables|Default|GetPlayer%20Unit))
      (bind _returnvalue (Utilities|Time|SetTimerbyEvent (delegate Custom|TryAttackEnemyInRange) (Variables|Default|GetAttack%20Speed) true))
      (Variables|Default|SetTryAttackTimer _returnvalue))))

(event Custom|HandleAttackCommand
  (params (AttackLocation :type Vector) (AttackTarget :type Actor%20Object%20Reference) (PlayerUnit :type Actor%20Object%20Reference) (AttackRange :type Float%20%28double-precision%29))
  (Utilities|FlowControl|Sequence
    (:then_0
      (Variables|Default|SetPlayer%20Unit PlayerUnit)
      (Variables|Default|SetAttackTarget AttackTarget)
      (Variables|Default|SetAttackLocation "0, 0, 0")
      (bind _commandqueue (Class|BIPlayerUnit|GetUnitCommandQueue(Message) PlayerUnit))
      (Variables|Default|SetCommand%20Queue _commandqueue))
    (:then_1
      (if (<= (Transformation|GetDistanceTo PlayerUnit AttackTarget) AttackRange)
        (Utilities|Array|Add (Variables|Default|GetCommand%20Queue) (Utilities|Struct|MakeF_UnitCommand "NewEnumerator1" (Variables|Default|GetAttackLocation) (Variables|Default|GetAttackTarget)))
        (else
          (Class|BIPlayerUnit|MoveCommand(Message) (Variables|Default|GetPlayer%20Unit) (Variables|Default|GetAttackLocation) (Variables|Default|GetAttackTarget)))))))

(event Custom|TryAttackEnemyInRange
  (Utilities|IsValid (Variables|Default|GetTargetActor)
    (:Is%20Valid
      (Utilities|Time|ClearandInvalidateTimerbyHandle (Variables|Default|GetLookForNearbyTargetTimer))
      (if (>= (Transformation|GetDistanceTo (Variables|Default|GetPlayer%20Unit) (.targetactor (Variables|Default|GetCurrent%20Command))) (Variables|Default|GetAttack%20Range))
        (Utilities|Time|ClearandInvalidateTimerbyHandle (Variables|Default|GetTryAttackTimer))
        (Utilities|Array|Add (Variables|Default|GetCommand%20Queue) (Utilities|Struct|MakeF_UnitCommand "NewEnumerator0" (Variables|Default|GetTargetLocation) 0))
        (Utilities|Array|Add (Variables|Default|GetCommand%20Queue) (Utilities|Struct|MakeF_UnitCommand "NewEnumerator1" "0.000000,0.000000,0.000000" (Variables|Default|GetTargetActor)))
        (Class|BIPlayerUnit|AddCommandstoQueue(Message) (Variables|Default|GetPlayer%20Unit) (Variables|Default|GetCommand%20Queue))
        (else
          (Game|Damage|ApplyDamage (Variables|Default|GetTargetActor) (Variables|Default|GetAttack%20Damage) (Variables|Default|GetAIController) 0))))
    (:Is%20Not%20Valid
      (Utilities|Time|ClearandInvalidateTimerbyHandle (Variables|Default|GetTryAttackTimer)))))