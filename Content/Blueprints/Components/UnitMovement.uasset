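; Movement component for player units that queues move commands and executes them through AI navigation.
; Move requests are added to the unit's command queue, then run with AIMoveTo, which rechecks the queue only when the move finishes.
; A separate helper finds reachable points near target actors: it projects a point short of the target onto the navmesh, falling back to a path endpoint, then a wider projection beyond the target.
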(event Custom|HandleMoveCommand
  (params (AIController :type AI%20Controller%20Object%20Reference) (TargetLocation :type Vector) (TargetActor :type Actor%20Object%20Reference) (PlayerUnit :type Actor%20Object%20Reference) (CommandQueue :type Array%20of%20F%20Unit%20Command%20Structures))
  (Variables|Default|SetPlayer%20Unit PlayerUnit)
  (Class|BIPlayerUnit|AddCommandstoQueue(Message) (Variables|Default|GetPlayer%20Unit) (Utilities|Array|MakeArray (Utilities|Struct|MakeF_UnitCommand "NewEnumerator0" TargetLocation TargetActor)))
  (Class|BIPlayerUnit|CheckCommandQueue(Message) (Variables|Default|GetPlayer%20Unit)))

(event Custom|ExecuteMoveCommand
  (params (AIController :type AI%20Controller%20Object%20Reference) (TargetLocation :type Vector) (TargetActor :type Actor%20Object%20Reference) (PlayerUnit :type Actor%20Object%20Reference))
  (AI|AIMoveTo AIController TargetLocation TargetActor 5.0 "Default" "Default" true true
    (:then
      (Development|PrintString "Move issued"))
    (:OnRequestFailed
      (Development|PrintString "On move failed"))
    (:OnMoveFinished
      (Development|PrintString "On move finished")
      (Class|BIPlayerUnit|CheckCommandQueue(Message) PlayerUnit))))

(fn FindValidLocationtoNavigate
  (params (PlayerUnit :type Actor%20Object%20Reference) (TargetLocation :type Vector) (TargetActor :type Actor%20Object%20Reference))
  (LocalVariables|SetUnit PlayerUnit)
  (Utilities|IsValid TargetActor
    (:Is%20Valid
      (LocalVariables|SetlocationToNavigate (Transformation|GetActorLocation TargetActor))
      (LocalVariables|SetDirectionToTarget (Class|KismetMathLibrary|VectorNormal2D (- (LocalVariables|GetlocationToNavigate) (Transformation|GetActorLocation (LocalVariables|GetUnit))) 0.0001))
      (bind _output_get (LocalVariables|SetPreferredTargetLocation (- (LocalVariables|GetlocationToNavigate) (* (LocalVariables|GetDirectionToTarget) (LocalVariables|GetDirectionToTargetDistanceOffset) 0.5))))
      (bind _output_get_2 (LocalVariables|SetNearestValidPoint (.ProjectedLocation (AI|Navigation|ProjectPointtoNavigation (Class|NavigationSystemV1|GetNavigationSystem) _output_get 0 0 (Math|Conversions|ToVector(Float) (LocalVariables|GetValidPointSearchRadius))))))
      (if (.ReturnValue (AI|Navigation|ProjectPointtoNavigation (Class|NavigationSystemV1|GetNavigationSystem) _output_get 0 0 (Math|Conversions|ToVector(Float) (LocalVariables|GetValidPointSearchRadius))))
        (return _output_get_2)
        (else
          (bind _returnvalue (Class|NavigationSystemV1|FindPathtoLocationSynchronously (Transformation|GetActorLocation (LocalVariables|GetUnit)) (LocalVariables|GetlocationToNavigate) 0 0))
          (if (Utilities|IsValid _returnvalue)
            (bind _output_get_3 (LocalVariables|SetFinalPathPoint (Utilities|Array|Get(acopy) (Variables|/Script/NavigationSystem.NavigationPath|GetPathPoints _returnvalue) (Utilities|Array|LastIndex (Variables|/Script/NavigationSystem.NavigationPath|GetPathPoints _returnvalue)))))
            (return _output_get_3)
            (else
              (bind _output_get_4 (LocalVariables|SetExpandedTargetLocation (+ (* (LocalVariables|GetDirectionToTarget) (LocalVariables|GetDirectionToTargetDistanceOffset)) (LocalVariables|GetlocationToNavigate))))
              (bind _output_get_5 (LocalVariables|SetNearestValidPoint (.ProjectedLocation (AI|Navigation|ProjectPointtoNavigation _output_get_4 0 0 (Math|Conversions|ToVector(Float) (* (LocalVariables|GetValidPointSearchRadius) (LocalVariables|GetValidPointSearchRadiusMultiplier)))))))
              (if (.ReturnValue (AI|Navigation|ProjectPointtoNavigation _output_get_4 0 0 (Math|Conversions|ToVector(Float) (* (LocalVariables|GetValidPointSearchRadius) (LocalVariables|GetValidPointSearchRadiusMultiplier)))))
                (return _output_get_5)
                (else
                  (Development|PrintString "All navigation attempts failed. Worker cannot reach the tree!" true true "(R=1.000000,G=0.000000,B=0.000000,A=1.000000)"))))))))
    (:Is%20Not%20Valid
      (return TargetLocation))))